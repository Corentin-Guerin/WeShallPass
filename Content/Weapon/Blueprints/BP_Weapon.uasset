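; BP_Weapon is a player pistol with Glock animations that handles firing, ammo and timed reloads from a reserve.
; Fire decrements ammo, plays randomized gunshot audio and animation, or a dry-fire sound when empty.
; A camera trace with random spread picks the impact point for a decal, while a tracer spawns at the muzzle.
; The follow-up muzzle-to-impact trace's result is unused, and no damage is applied.
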(event `self.Fire`
  (if (> (`self.Ammocount`) 0)
    (`self.AmmoCheck`)
    (bind (_muzzel_lock _impactpoint) (`self.LineTrace`))
    (`self.SpawnDecalTracer` _muzzel_lock _impactpoint _impactpoint)
    (else
      (`GameplayStatics.PlaySoundAtLocation` "/Game/Weapon/Sounds/DryFire.DryFire" (`SceneComponent.K2_GetComponentLocation` (`/Game/Blueprints/Player/BP_My_Player.Camera` (cast `/Game/Blueprints/Player/BP_My_Player` (`GameplayStatics.GetPlayerCharacter` 0) :!pure true))) (struct) 1.0 1.0 0.0 null null null))))

(event `self.AddMunitions`
  (set `self.MaxAmmo` (+ (`self.MaxAmmo`) (`self.AmmoChargeur`))))

(event `self.Reload`
  (`SkeletalMeshComponent.PlayAnimation` (`self.PrimaryWeapon`) "/Game/Animation/Weapon/Glock_Reload_anim_Montage.Glock_Reload_anim_Montage" false)
  (`KismetSystemLibrary.Delay` (`self.ReloadTime`))
  (if (> (`self.MaxAmmo`) (`self.AmmoChargeur`))
    (set `self.MaxAmmo` (- (+ (`self.MaxAmmo`) (`self.Ammocount`)) (`self.AmmoChargeur`)))
    (set `self.Ammocount` (`self.AmmoChargeur`))
    (else
      (set `self.MaxAmmo` (+ (`self.MaxAmmo`) (`self.Ammocount`)))
      (if (< (`self.MaxAmmo`) (`self.AmmoChargeur`))
        (set `self.Ammocount` (`self.MaxAmmo`))
        (set `self.MaxAmmo` 0)
        (else
          (set `self.MaxAmmo` (- (`self.MaxAmmo`) (`self.AmmoChargeur`)))
          (set `self.Ammocount` (`self.AmmoChargeur`)))))))

(fn `AmmoCheck`
  (bind _returnvalue (`KismetMathLibrary.RandomFloatInRange` 0.7 1.2))
  (`/Engine/EditorBlueprintResources/StandardMacros.DecrementInt` (`self.Ammocount`)
    (:`  `
      (if (not (`/Game/Blueprints/Player/BP_My_Player.IsReloading` (cast `/Game/Blueprints/Player/BP_My_Player` (`GameplayStatics.GetPlayerCharacter` 0) :!pure true)))
        (`GameplayStatics.PlaySoundAtLocation` "/Game/Weapon/Sounds/Gunshot.Gunshot" (`SceneComponent.K2_GetComponentLocation` (`/Game/Blueprints/Player/BP_My_Player.Camera` (cast `/Game/Blueprints/Player/BP_My_Player` (`GameplayStatics.GetPlayerCharacter` 0) :!pure true))) (struct) (+ _returnvalue 2.5) _returnvalue 0.0 null null null)
        (`SkeletalMeshComponent.PlayAnimation` (`self.PrimaryWeapon`) "/Game/Animation/Weapon/Glock_Fire_anim_Montage.Glock_Fire_anim_Montage" false)))))

(fn `LineTrace`
  (returns (`Muzzel Lock` :type "Vector Structure") (ImpactPoint :type "Vector Structure"))
  (bind _bulletspread (`self.BulletSpread`))
  (bind _returnvalue (`SceneComponent.K2_GetComponentLocation` (`self.Muzzle`)))
  (bind _returnvalue_2 (* _bulletspread -1.0))
  (bind _camera (`/Game/Blueprints/Player/BP_My_Player.Camera` (cast `/Game/Blueprints/Player/BP_My_Player` (`GameplayStatics.GetPlayerCharacter` 0) :!pure true)))
  (bind _returnvalue_3 (`SceneComponent.K2_GetComponentLocation` _camera))
  (bind _outhit (`KismetSystemLibrary.LineTraceSingle` _returnvalue_3 (+ (+ (* (`SceneComponent.GetForwardVector` _camera) 20000.0) _returnvalue_3) (`KismetMathLibrary.MakeVector` (`KismetMathLibrary.RandomFloatInRange` _returnvalue_2 _bulletspread) (`KismetMathLibrary.RandomFloatInRange` _returnvalue_2 _bulletspread) (`KismetMathLibrary.RandomFloatInRange` _returnvalue_2 _bulletspread))) "TraceTypeQuery1")) ; Camera Shot
  (bind (_bblockinghit _binitialoverlap _time _distance _location _impactpoint) (`GameplayStatics.BreakHitResult` _outhit))
  (`KismetSystemLibrary.LineTraceSingle` :`Start` _returnvalue :`End` _impactpoint :`TraceChannel` "TraceTypeQuery1" :`TraceColor` (struct :`R` 1.0 :`B` 0.043706 :`A` 1.0)) ; GUN Shot
  (return _returnvalue _impactpoint))

(fn `SpawnDecalTracer`
  (params (Location :type "Vector Structure") (SpawnTransformLoc :type "Vector Structure") (ImpactPoint :type "Vector Structure"))
  (`|SpawnActorFromClass` "/Game/Weapon/Blueprints/BP_DecalBullet.BP_DecalBullet_C" (`KismetMathLibrary.MakeTransform` SpawnTransformLoc (`KismetMathLibrary.MakeRotFromX` ImpactPoint) (0.025 0.025 0.025)) "Undefined" "OverrideRootScale" null null)
  (`|SpawnActorFromClass` "/Game/Weapon/Blueprints/BP_TracerBullet.BP_TracerBullet_C" (`KismetMathLibrary.MakeTransform` Location (`SceneComponent.K2_GetComponentRotation` (`/Game/Blueprints/Player/BP_My_Player.Camera` (cast `/Game/Blueprints/Player/BP_My_Player` (`GameplayStatics.GetPlayerCharacter` 0) :!pure true))) (0.05 0.05 0.05)) "Undefined" "OverrideRootScale" null null)
  (return))

(fn `UserConstructionScript`
  (`parent.UserConstructionScript`)
  (set `self.MaxAmmo` 32)
  (set `self.Ammocount` 8)
  (set `self.AmmoChargeur` 8)
  (set `self.ReloadTime` 2.0)
  (set `self.BulletSpread` 175.0))