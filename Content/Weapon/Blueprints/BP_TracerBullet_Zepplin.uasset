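; Zeppelin tracer bullet actor that kills the player on contact and bursts apart on any sphere overlap.
; An overlap calls PlayerDeath on BP_My_Player, hides the static mesh and adds a destructible component in its place.
; After a short delay it fires a radial impulse, activates particles and plays an explosion sound at the world origin.
; Several seconds later it removes the destructible and destroys itself.
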(event `self.Sphere.OnComponentBeginOverlap`
  (params (OverlappedComponent :type "PrimitiveComponent Object Reference") (OtherActor :type "Actor Object Reference") (OtherComp :type "PrimitiveComponent Object Reference") (OtherBodyIndex :type Integer) (bFromSweep :type Boolean) (SweepResult :type "HitResult Structure (by ref)"))
  (bind _asbp_my_player (cast `/Game/Blueprints/Player/BP_My_Player` OtherActor)
    (:`then`
      (`/Game/Blueprints/Player/BP_My_Player.PlayerDeath` _asbp_my_player))
    (:`CastFailed`
      _))
  (`SceneComponent.SetVisibility` (`self.StaticMesh`) false false)
  (bind _returnvalue (`AddComponent|NODE_AddDestructibleComponent-0` :`RelativeTransform` (`KismetMathLibrary.MakeTransform` (0.0 0.0 25.0) (struct :`Pitch` 90.0))))
  (`KismetSystemLibrary.Delay` 0.2)
  (`RadialForceComponent.FireImpulse` (`self.RadialForce`))
  (`ActorComponent.Activate` (`self.ParticleSystem`) false)
  (`GameplayStatics.PlaySoundAtLocation` "/Game/StarterContent/Audio/Explosion01.Explosion01" (0.0 0.0 0.0) (struct) 0.5 1.0 0.0 null null null)
  (`KismetSystemLibrary.Delay` 5.0)
  (`ActorComponent.K2_DestroyComponent` _returnvalue)
  (`self.K2_DestroyActor`))

(fn `UserConstructionScript`)