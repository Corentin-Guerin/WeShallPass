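; Searchlight obstacle that sweeps on a timeline and flags the player as discovered when they enter its cone.
; While triggered or during a chase, the sweep stops, the lights change color and the spotlight tracks the player.
; A visibility trace keeps detection active, clearing it after a delay when the player is not hit.
; A tracer bullet entering its sphere temporarily hides the lights, then resets detection.
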(event `self.ReceiveTick`
  (params (DeltaSeconds :type "Float (single-precision)"))
  (bind _myplayercharactere (`/Game/Blueprints/Player/FuctionLibrary/BFFL_CallPLayerController.CallMyPlayerCharactere`))
  (bind _returnvalue (`SceneComponent.K2_GetComponentLocation` (`self.SpotLight`)))
  (bind _returnvalue_2 (`SceneComponent.K2_GetComponentLocation` (`Actor.RootComponent` (`GameplayStatics.GetPlayerCharacter` 0))))
  (if (and (not (`/Game/Blueprints/Player/BP_My_Player.IsChase` (`/Game/Blueprints/Player/FuctionLibrary/BFFL_CallPLayerController.CallMyPlayerCharactere`))) (not (`self.IsTrigger`)))
    (bind (_direction _newtrack_0) (`Timeline|Timeline_0` :!label _label)
      (:`Update`
        (`SceneComponent.K2_SetWorldRotation` (`self.DefaultSceneRoot`) (`KismetMathLibrary.MakeRotator` 0.0 0.0 _newtrack_0) false false)
        (if (not (`self.CourseReset`))
          (`LightComponent.SetLightColor` (`self.PointLight`) (`self.DefaultColor`) true)
          (`LightComponent.SetLightColor` (`self.SpotLight`) (`self.DefaultColor`) true)
          (`SceneComponent.K2_SetWorldRotation` (`self.PointLight`) (`self.DefaultSpotLightRot`) false false)
          (`SceneComponent.K2_SetWorldRotation` (`self.SpotLight`) (`self.DefaultSpotLightRot`) false false)
          (set `self.CourseReset` true))))
    (else
      (set `self.CourseReset` false)
      (`|ExecutionSequence`
        (:`then_0`
          (goto _label :!via `Stop`))
        (:`then_1`
          (`SceneComponent.K2_SetWorldRotation` (`self.SpotLight`) (`KismetMathLibrary.FindLookAtRotation` (`SceneComponent.K2_GetComponentLocation` (`self.DefaultSceneRoot`)) (`SceneComponent.K2_GetComponentLocation` (`Character.CapsuleComponent` (`/Game/Blueprints/Player/FuctionLibrary/BFFL_CallPLayerController.CallMyPlayerCharactere`)))) true true))
        (:`then_2`
          (`LightComponent.SetLightColor` (`self.PointLight`) (`self.Detect_Color`) true)
          (`LightComponent.SetLightColor` (`self.SpotLight`) (`self.Detect_Color`) true))
        (:`then_3`
          (bind _outhit (`KismetSystemLibrary.LineTraceSingle` _returnvalue (+ _returnvalue_2 (* (`KismetMathLibrary.Normal` (- _returnvalue_2 _returnvalue)) 100.0)) "TraceTypeQuery1")) ; Camera Shot
          (cast `/Game/Blueprints/Player/BP_My_Player` (`.HitActor` (`GameplayStatics.BreakHitResult` _outhit))
            (:`then`
              (set `/Game/Blueprints/Player/BP_My_Player.IsDiscover` true _myplayercharactere)
              (set `self.IsTrigger` true))
            (:`CastFailed`
              (`KismetSystemLibrary.Delay` 5.0)
              (set `/Game/Blueprints/Player/BP_My_Player.IsDiscover` false _myplayercharactere)
              (set `self.IsTrigger` false))))))))

(event `self.ReceiveBeginPlay`
  (set `self.DefaultSpotLightRot` (`SceneComponent.K2_GetComponentRotation` (`self.SpotLight`))))

(event `self.Cone.OnComponentBeginOverlap`
  (params (OverlappedComponent :type "PrimitiveComponent Object Reference") (OtherActor :type "Actor Object Reference") (OtherComp :type "PrimitiveComponent Object Reference") (OtherBodyIndex :type Integer) (bFromSweep :type Boolean) (SweepResult :type "HitResult Structure (by ref)"))
  (cast `/Game/Blueprints/Player/BP_My_Player` OtherActor)
  (if (not (`self.IsTrigger`))
    (set `/Game/Blueprints/Player/BP_My_Player.IsDiscover` true (`/Game/Blueprints/Player/FuctionLibrary/BFFL_CallPLayerController.CallMyPlayerCharactere`))
    (set `self.IsTrigger` true)))

(event `self.Sphere.OnComponentBeginOverlap`
  (params (OverlappedComponent :type "PrimitiveComponent Object Reference") (OtherActor :type "Actor Object Reference") (OtherComp :type "PrimitiveComponent Object Reference") (OtherBodyIndex :type Integer) (bFromSweep :type Boolean) (SweepResult :type "HitResult Structure (by ref)"))
  (cast `/Game/Weapon/Blueprints/BP_TracerBullet` OtherActor)
  (`SceneComponent.SetVisibility` (`self.PointLight`) false false)
  (`SceneComponent.SetVisibility` (`self.SpotLight`) false false)
  (`KismetSystemLibrary.Delay` 5.0)
  (set `/Game/Blueprints/Player/BP_My_Player.IsDiscover` false (`/Game/Blueprints/Player/FuctionLibrary/BFFL_CallPLayerController.CallMyPlayerCharactere`))
  (`SceneComponent.SetVisibility` (`self.PointLight`) true false)
  (`SceneComponent.SetVisibility` (`self.SpotLight`) true false)
  (`SceneComponent.K2_SetWorldRotation` (`self.PointLight`) (`self.DefaultSpotLightRot`) false false)
  (`SceneComponent.K2_SetWorldRotation` (`self.SpotLight`) (`self.DefaultSpotLightRot`) false false)
  (`LightComponent.SetLightColor` (`self.PointLight`) (`self.DefaultColor`) true)
  (`LightComponent.SetLightColor` (`self.SpotLight`) (`self.DefaultColor`) true)
  (set `self.IsTrigger` false))

(fn `UserConstructionScript`)