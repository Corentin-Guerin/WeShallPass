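; Searchlight mech with two projectors that sweep back and forth until the player is detected or chased.
; Cone overlaps raise the alert, turning lights to the detect color and aiming spotlights and body at the player.
; Line traces from both projectors check cover, clearing the alert after a delay when hidden.
; Tracer bullets temporarily knock out each light; losing both halts body tracking, and their restoration clears the alert.
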(event `self.ReceiveBeginPlay`
  (set `self.DefautRotProjGauche` (`SceneComponent.K2_GetComponentRotation` (`self.Projecteur Gauche`)))
  (set `self.DefautRotProjDroite` (`SceneComponent.K2_GetComponentRotation` (`self.Projecteur Droite`)))
  (set `self.DefautRotMeca` (`SceneComponent.K2_GetComponentRotation` (`self.Meca`))))

(event `self.ReceiveTick`
  (params (DeltaSeconds :type "Float (single-precision)"))
  (bind _myplayercharactere (`/Game/Blueprints/Player/FuctionLibrary/BFFL_CallPLayerController.CallMyPlayerCharactere`))
  (bind _myplayercharactere_2 (`/Game/Blueprints/Player/FuctionLibrary/BFFL_CallPLayerController.CallMyPlayerCharactere`))
  (bind _spotlight (`self.SpotLight`))
  (bind _spotlight1 (`self.SpotLight1`))
  (bind _meca (`self.Meca`))
  (bind (_relativerotation_roll _relativerotation_pitch _relativerotation_yaw) (`KismetMathLibrary.BreakRotator` (`SceneComponent.RelativeRotation` (`self.Projecteur Gauche`))))
  (bind (_relativerotation_roll_2 _relativerotation_pitch_2 _relativerotation_yaw_2) (`KismetMathLibrary.BreakRotator` (`SceneComponent.RelativeRotation` (`self.Projecteur Gauche`))))
  (bind (_returnvalue_roll _returnvalue_pitch _returnvalue_yaw) (`KismetMathLibrary.BreakRotator` (`KismetMathLibrary.FindLookAtRotation` (`SceneComponent.K2_GetComponentLocation` _meca) (`SceneComponent.K2_GetComponentLocation` (`Character.CapsuleComponent` (`/Game/Blueprints/Player/FuctionLibrary/BFFL_CallPLayerController.CallMyPlayerCharactere`))))))
  (if (and (not (`/Game/Blueprints/Player/BP_My_Player.IsChase` _myplayercharactere_2)) (not (`/Game/Blueprints/Player/BP_My_Player.IsDiscover` _myplayercharactere_2)) (not (`self.IsTrigger`)))
    (if (>= _relativerotation_yaw_2 (`self.RotationMax`))
      (set `self.Addrotation` -0.2)
      (elif (<= _relativerotation_yaw (`self.RotationMin`))
        (set `self.Addrotation` 0.2)))
    (`SceneComponent.K2_AddRelativeRotation` (`self.Projecteur Droite`) (`KismetMathLibrary.MakeRotator` 0.0 0.0 (`self.Addrotation`)) false false)
    (`SceneComponent.K2_AddRelativeRotation` (`self.Projecteur Gauche`) (`KismetMathLibrary.MakeRotator` 0.0 0.0 (`self.Addrotation`)) false false)
    (`SceneComponent.K2_AddRelativeRotation` (`self.StaticMesh`) (`KismetMathLibrary.MakeRotator` 0.0 0.0 (`self.Addrotation`)) false false)
    (`SceneComponent.K2_AddRelativeRotation` (`self.StaticMesh1`) (`KismetMathLibrary.MakeRotator` 0.0 0.0 (`self.Addrotation`)) false false)
    (if (not (`self.ResetCourse`))
      (`LightComponent.SetLightColor` (`self.PointLight`) (`self.DefaultColor`) true)
      (`LightComponent.SetLightColor` (`self.PointLight1`) (`self.DefaultColor`) true)
      (`LightComponent.SetLightColor` (`self.SpotLight1`) (`self.DefaultColor`) true)
      (`LightComponent.SetLightColor` (`self.SpotLight`) (`self.DefaultColor`) true)
      (`SceneComponent.K2_SetWorldRotation` (`self.Meca`) (`self.DefautRotMeca`) false false)
      (`SceneComponent.K2_SetWorldRotation` (`self.SpotLight1`) (`self.DefautRotProjDroite`) false false)
      (`SceneComponent.K2_SetWorldRotation` (`self.PointLight1`) (`self.DefautRotProjDroite`) false false)
      (`SceneComponent.K2_SetWorldRotation` (`self.SpotLight`) (`self.DefautRotProjGauche`) false false)
      (`SceneComponent.K2_SetWorldRotation` (`self.PointLight`) (`self.DefautRotProjGauche`) false false)
      (set `self.ResetCourse` true))
    (else
      (set `self.ResetCourse` false)
      (`|ExecutionSequence`
        (:`then_0`
          (`SceneComponent.K2_SetWorldRotation` _spotlight (`KismetMathLibrary.FindLookAtRotation` (`SceneComponent.K2_GetComponentLocation` _spotlight) (`SceneComponent.K2_GetComponentLocation` (`Character.CapsuleComponent` (`/Game/Blueprints/Player/FuctionLibrary/BFFL_CallPLayerController.CallMyPlayerCharactere`)))) true true)
          (`SceneComponent.K2_SetWorldRotation` _spotlight1 (`KismetMathLibrary.FindLookAtRotation` (`SceneComponent.K2_GetComponentLocation` _spotlight1) (`SceneComponent.K2_GetComponentLocation` (`Character.CapsuleComponent` (`/Game/Blueprints/Player/FuctionLibrary/BFFL_CallPLayerController.CallMyPlayerCharactere`)))) true true)
          (if (or (not (`self.Spot1Destroy`)) (not (`self.Spot2Destroy`)))
            (`SceneComponent.K2_SetWorldRotation` _meca (`KismetMathLibrary.MakeRotator` 0.0 0.0 (+ _returnvalue_yaw 90.0)) true true)))
        (:`then_1`
          (`LightComponent.SetLightColor` (`self.SpotLight`) (`self.DetectColor`) true)
          (`LightComponent.SetLightColor` (`self.PointLight`) (`self.DetectColor`) true)
          (`LightComponent.SetLightColor` (`self.PointLight1`) (`self.DetectColor`) true)
          (`LightComponent.SetLightColor` (`self.SpotLight1`) (`self.DetectColor`) true))
        (:`then_2`
          (bind _hitactor (`self.Detectiondujoueur` (`self.Projecteur Droite`)))
          (cast `/Game/Blueprints/Player/BP_My_Player` _hitactor
            (:`then`
              (set `self.Joueurcacher` false))
            (:`CastFailed`
              (set `self.Joueurcacher` true)))
          (bind _hitactor_2 (`self.Detectiondujoueur` (`self.Projecteur Gauche`)))
          (cast `/Game/Blueprints/Player/BP_My_Player` _hitactor_2
            (:`then`
              (set `self.Joueurcacher` false))
            (:`CastFailed`
              (set `self.Joueurcacher` true)))
          (if (not (`self.Joueurcacher`))
            (set `/Game/Blueprints/Player/BP_My_Player.IsDiscover` true _myplayercharactere)
            (set `self.IsTrigger` true)
            (else
              (`KismetSystemLibrary.Delay` 5.0)
              (set `/Game/Blueprints/Player/BP_My_Player.IsDiscover` false _myplayercharactere)
              (set `self.IsTrigger` false))))))))

(event `self.ConeDroite.OnComponentBeginOverlap`
  (params (OverlappedComponent :type "PrimitiveComponent Object Reference") (OtherActor :type "Actor Object Reference") (OtherComp :type "PrimitiveComponent Object Reference") (OtherBodyIndex :type Integer) (bFromSweep :type Boolean) (SweepResult :type "HitResult Structure (by ref)"))
  (cast `/Game/Blueprints/Player/BP_My_Player` OtherActor)
  (if (not (`self.Joueurcacher`))
    (set `self.IsTrigger` true)
    (set `/Game/Blueprints/Player/BP_My_Player.IsDiscover` true (`/Game/Blueprints/Player/FuctionLibrary/BFFL_CallPLayerController.CallMyPlayerCharactere`))))

(event `self.Cone Gauche.OnComponentBeginOverlap`
  (params (OverlappedComponent :type "PrimitiveComponent Object Reference") (OtherActor :type "Actor Object Reference") (OtherComp :type "PrimitiveComponent Object Reference") (OtherBodyIndex :type Integer) (bFromSweep :type Boolean) (SweepResult :type "HitResult Structure (by ref)"))
  (cast `/Game/Blueprints/Player/BP_My_Player` OtherActor)
  (if (not (`self.Joueurcacher`))
    (set `self.IsTrigger` true)
    (set `/Game/Blueprints/Player/BP_My_Player.IsDiscover` true (`/Game/Blueprints/Player/FuctionLibrary/BFFL_CallPLayerController.CallMyPlayerCharactere`))))

(event `self.Sphere.OnComponentBeginOverlap`
  (params (OverlappedComponent :type "PrimitiveComponent Object Reference") (OtherActor :type "Actor Object Reference") (OtherComp :type "PrimitiveComponent Object Reference") (OtherBodyIndex :type Integer) (bFromSweep :type Boolean) (SweepResult :type "HitResult Structure (by ref)"))
  (bind _spot1destroy (`self.Spot1Destroy`))
  (bind _spot2destroy (`self.Spot2Destroy`))
  (cast `/Game/Weapon/Blueprints/BP_TracerBullet` OtherActor)
  (`SceneComponent.SetVisibility` (`self.PointLight`) false false)
  (`SceneComponent.SetVisibility` (`self.SpotLight`) false false)
  (set `self.Spot1Destroy` true)
  (if (and _spot1destroy _spot2destroy) :!label _label
    (`KismetSystemLibrary.Delay` 5.0 :!label _label_2)
    (`SceneComponent.SetVisibility` (`self.PointLight`) true false)
    (`SceneComponent.SetVisibility` (`self.SpotLight`) true false)
    (`SceneComponent.SetVisibility` (`self.SpotLight1`) true false)
    (`SceneComponent.SetVisibility` (`self.PointLight1`) true false)
    (set `self.Spot1Destroy` false)
    (set `self.Spot2Destroy` false)
    (set `/Game/Blueprints/Player/BP_My_Player.IsDiscover` false (`/Game/Blueprints/Player/FuctionLibrary/BFFL_CallPLayerController.CallMyPlayerCharactere`))
    (set `self.IsTrigger` false)
    (elif _spot1destroy
      (`KismetSystemLibrary.Delay` 5.0)
      (if (not (`self.Spot2Destroy`))
        (`SceneComponent.SetVisibility` (`self.PointLight`) true false)
        (`SceneComponent.SetVisibility` (`self.SpotLight`) true false)
        (set `self.Spot1Destroy` false)
        (else
          (goto _label_2)))
      (elif _spot2destroy
        (`KismetSystemLibrary.Delay` 5.0)
        (if (not (`self.Spot1Destroy`))
          (`SceneComponent.SetVisibility` (`self.PointLight1`) true false)
          (`SceneComponent.SetVisibility` (`self.SpotLight1`) true false)
          (set `self.Spot2Destroy` false)
          (else
            (goto _label_2)))))))

(event `self.Sphere1.OnComponentBeginOverlap`
  (params (OverlappedComponent :type "PrimitiveComponent Object Reference") (OtherActor :type "Actor Object Reference") (OtherComp :type "PrimitiveComponent Object Reference") (OtherBodyIndex :type Integer) (bFromSweep :type Boolean) (SweepResult :type "HitResult Structure (by ref)"))
  (cast `/Game/Weapon/Blueprints/BP_TracerBullet` OtherActor)
  (`SceneComponent.SetVisibility` (`self.PointLight1`) false false)
  (`SceneComponent.SetVisibility` (`self.SpotLight1`) false false)
  (set `self.Spot2Destroy` true)
  (goto _label))

(fn `Detectiondujoueur`
  (params (self2 :type "SceneComponent Object Reference"))
  (returns (HitActor :type "Actor Object Reference"))
  (bind _returnvalue (`SceneComponent.K2_GetComponentLocation` self2))
  (bind _returnvalue_2 (`SceneComponent.K2_GetComponentLocation` (`Actor.RootComponent` (`GameplayStatics.GetPlayerCharacter` 0))))
  (bind _outhit (`KismetSystemLibrary.LineTraceSingle` :`Start` _returnvalue :`End` (+ _returnvalue_2 (* (`KismetMathLibrary.Normal` (- _returnvalue_2 _returnvalue)) 100.0)) :`TraceChannel` "TraceTypeQuery1" :`bIgnoreSelf` false)) ; Camera Shot
  (return (`.HitActor` (`GameplayStatics.BreakHitResult` _outhit))))

(fn `UserConstructionScript`)