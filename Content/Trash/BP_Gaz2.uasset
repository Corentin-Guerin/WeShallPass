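; BP_Gaz2 is a gas hazard zone that fades a screen effect on the player and kills them if they stay inside.
; GazZone overlap begin and end set the player's IsInGaz flag and, after a short delay, play or reverse two timelines.
; These drive R_Fade and T_Fade on a dynamic material instance for the player's GazPlane.
; When the R_Fade timeline finishes with IsInGaz still true, the player's IsDead is set.
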(event `InGaz`
  (bind _myplayercharactere (`/Game/Blueprints/Player/FuctionLibrary/BFFL_CallPLayerController.CallMyPlayerCharactere`))
  (`KismetSystemLibrary.Delay` 0.2)
  (bind _returnvalue (`PrimitiveComponent.CreateDynamicMaterialInstance` (`/Game/Blueprints/Player/BP_My_Player.GazPlane` (`/Game/Blueprints/Player/FuctionLibrary/BFFL_CallPLayerController.CallMyPlayerCharactere`)) 0 "/Game/Textures/Material/M_GazScreenPlane.M_GazScreenPlane" "None"))
  (`|ExecutionSequence`
    (:`then_0`
      (bind (_direction _newtrack_0) (`Timeline|Timeline_0` :!label _label)
        (:`Update`
          (`MaterialInstanceDynamic.SetScalarParameterValue` _returnvalue "R_Fade" _newtrack_0))
        (:`Finished`
          (if (`/Game/Blueprints/Player/BP_My_Player.IsInGaz` _myplayercharactere)
            (set `/Game/Blueprints/Player/BP_My_Player.IsDead` true _myplayercharactere)))))
    (:`then_1`
      (bind (_direction_2 _newtrack_0_2) (`Timeline|Timeline_1` :!label _label_2)
        (:`Update`
          (`MaterialInstanceDynamic.SetScalarParameterValue` _returnvalue "T_Fade" _newtrack_0_2))))))

(event `IsNotInGaz`
  (`KismetSystemLibrary.Delay` 0.2)
  (`PrimitiveComponent.CreateDynamicMaterialInstance` (`/Game/Blueprints/Player/BP_My_Player.GazPlane` (`/Game/Blueprints/Player/FuctionLibrary/BFFL_CallPLayerController.CallMyPlayerCharactere`)) 0 "/Game/Textures/Material/M_GazScreenPlane.M_GazScreenPlane" "None")
  (`|ExecutionSequence`
    (:`then_0`
      (goto _label :!via `Reverse`))
    (:`then_1`
      (goto _label_2 :!via `Reverse`))))

(event `self.GazZone.OnComponentBeginOverlap`
  (params (OverlappedComponent :type "PrimitiveComponent Object Reference") (OtherActor :type "Actor Object Reference") (OtherComp :type "PrimitiveComponent Object Reference") (OtherBodyIndex :type Integer) (bFromSweep :type Boolean) (SweepResult :type "HitResult Structure (by ref)"))
  (cast `/Game/Blueprints/Player/BP_My_Player` OtherActor)
  (set `/Game/Blueprints/Player/BP_My_Player.IsInGaz` true (`/Game/Blueprints/Player/FuctionLibrary/BFFL_CallPLayerController.CallMyPlayerCharactere`))
  (`self.InGaz`))

(event `self.GazZone.OnComponentEndOverlap`
  (params (OverlappedComponent :type "PrimitiveComponent Object Reference") (OtherActor :type "Actor Object Reference") (OtherComp :type "PrimitiveComponent Object Reference") (OtherBodyIndex :type Integer))
  (cast `/Game/Blueprints/Player/BP_My_Player` OtherActor)
  (set `/Game/Blueprints/Player/BP_My_Player.IsInGaz` false (`/Game/Blueprints/Player/FuctionLibrary/BFFL_CallPLayerController.CallMyPlayerCharactere`))
  (`self.IsNotInGaz`))

(fn `UserConstructionScript`)