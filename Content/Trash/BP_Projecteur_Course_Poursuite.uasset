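; BP_Projecteur_Course_Poursuite is a searchlight that sweeps until triggered, then tracks the player, apparently for a chase sequence.
; While idle, Tick plays a timeline that drives the root's yaw.
; FocusPlayer, with no caller in this graph, flags detection: Tick stops the timeline, applies the detect color and aims the spotlight at the player's capsule.
; ResteProjecteur clears the flag, restoring default color and the rotation saved at BeginPlay.
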(event `self.ReceiveBeginPlay`
  (set `self.DefaultSpotLightRot` (`SceneComponent.K2_GetComponentRotation` (`self.SpotLight`))))

(event `ResteProjecteur`
  (set `self.IsTrigger` false)
  (`LightComponent.SetLightColor` (`self.PointLight`) (`self.DefaultColor`) true)
  (`LightComponent.SetLightColor` (`self.SpotLight`) (`self.DefaultColor`) true)
  (`SceneComponent.K2_SetWorldRotation` (`self.PointLight`) (`self.DefaultSpotLightRot`) false false)
  (`SceneComponent.K2_SetWorldRotation` (`self.SpotLight`) (`self.DefaultSpotLightRot`) false false))

(event `self.ReceiveTick`
  (params (DeltaSeconds :type "Float (single-precision)"))
  (if (not (`self.IsTrigger`))
    (bind (_direction _newtrack_0) (`Timeline|Timeline_0` :!label _label)
      (:`Update`
        (`SceneComponent.K2_SetWorldRotation` (`self.DefaultSceneRoot`) (`KismetMathLibrary.MakeRotator` 0.0 0.0 _newtrack_0) false false)))
    (else
      (`|ExecutionSequence`
        (:`then_0`
          (goto _label :!via `Stop`))
        (:`then_1`
          (`LightComponent.SetLightColor` (`self.PointLight`) (`self.Detect_Color`) true)
          (`LightComponent.SetLightColor` (`self.SpotLight`) (`self.Detect_Color`) true))
        (:`then_2`
          (`SceneComponent.K2_SetWorldRotation` (`self.SpotLight`) (`KismetMathLibrary.FindLookAtRotation` (`SceneComponent.K2_GetComponentLocation` (`self.DefaultSceneRoot`)) (`SceneComponent.K2_GetComponentLocation` (`Character.CapsuleComponent` (`/Game/Blueprints/Player/FuctionLibrary/BFFL_CallPLayerController.CallMyPlayerCharactere`)))) true true))))))

(event `FocusPlayer`
  (set `self.IsTrigger` true))

(fn `UserConstructionScript`)