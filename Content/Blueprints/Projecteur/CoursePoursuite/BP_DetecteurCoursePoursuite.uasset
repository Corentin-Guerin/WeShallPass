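; Chase-sequence detector actor that toggles the player's chase state through trigger volumes.
; Two start triggers set IsChase to true on an overlapping BP_My_Player, and two end triggers set it back to false.
; Disconnected nodes that would also set IsDiscover remain in the graph but never run.
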(event `self.TriggerdebutCourse.OnComponentBeginOverlap`
  (params (OverlappedComponent :type "PrimitiveComponent Object Reference") (OtherActor :type "Actor Object Reference") (OtherComp :type "PrimitiveComponent Object Reference") (OtherBodyIndex :type Integer) (bFromSweep :type Boolean) (SweepResult :type "HitResult Structure (by ref)"))
  (bind _asbp_my_player (cast `/Game/Blueprints/Player/BP_My_Player` OtherActor))
  (set `/Game/Blueprints/Player/BP_My_Player.IsChase` true _asbp_my_player))

(event `self.TriggerfinCourse.OnComponentBeginOverlap`
  (params (OverlappedComponent :type "PrimitiveComponent Object Reference") (OtherActor :type "Actor Object Reference") (OtherComp :type "PrimitiveComponent Object Reference") (OtherBodyIndex :type Integer) (bFromSweep :type Boolean) (SweepResult :type "HitResult Structure (by ref)"))
  (bind _asbp_my_player (cast `/Game/Blueprints/Player/BP_My_Player` OtherActor))
  (set `/Game/Blueprints/Player/BP_My_Player.IsChase` false _asbp_my_player))

(event `self.TriggerdebutCourse2.OnComponentBeginOverlap`
  (params (OverlappedComponent :type "PrimitiveComponent Object Reference") (OtherActor :type "Actor Object Reference") (OtherComp :type "PrimitiveComponent Object Reference") (OtherBodyIndex :type Integer) (bFromSweep :type Boolean) (SweepResult :type "HitResult Structure (by ref)"))
  (bind _asbp_my_player (cast `/Game/Blueprints/Player/BP_My_Player` OtherActor))
  (set `/Game/Blueprints/Player/BP_My_Player.IsChase` true _asbp_my_player))

(event `self.TriggerfinCourse2.OnComponentBeginOverlap`
  (params (OverlappedComponent :type "PrimitiveComponent Object Reference") (OtherActor :type "Actor Object Reference") (OtherComp :type "PrimitiveComponent Object Reference") (OtherBodyIndex :type Integer) (bFromSweep :type Boolean) (SweepResult :type "HitResult Structure (by ref)"))
  (bind _asbp_my_player (cast `/Game/Blueprints/Player/BP_My_Player` OtherActor))
  (set `/Game/Blueprints/Player/BP_My_Player.IsChase` false _asbp_my_player))

(fn `UserConstructionScript`)