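; BP_Projecteur_Menu is a spotlight projector, apparently a menu variant, that rotates on its own.
; Tick plays a timeline that drives the yaw of its Scene component, and BeginPlay stores the SpotLight's initial world rotation.
; Leftover unconnected chains would set the player's IsDiscover and IsTrigger, then call Sound to start or stop an alarm through SoundManager.
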(event `self.ReceiveTick`
  (params (DeltaSeconds :type "Float (single-precision)"))
  (bind (_direction _newtrack_0) (`Timeline|Timeline_0`)
    (:`Update`
      (`SceneComponent.K2_SetRelativeRotation` (`self.Scene`) (`KismetMathLibrary.MakeRotator` 0.0 0.0 _newtrack_0) false false))))

(event `self.ReceiveBeginPlay`
  (set `self.DefaultSpotLightRot` (`SceneComponent.K2_GetComponentRotation` (`self.SpotLight`))))

(fn `Sound`
  (bind _soundmanager (`self.SoundManager`))
  (if (`self.IsTrigger`)
    (`/Game/Blueprints/Sounds/BPC_SoundManager.PlaySound` _soundmanager (`self.SonAlarme`) (`SceneComponent.K2_GetComponentLocation` _soundmanager))
    (else
      (`/Game/Blueprints/Sounds/BPC_SoundManager.StopSound` _soundmanager))))

(fn `UserConstructionScript`)