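; BP_SavePoint is a checkpoint actor that records player progress for respawning.
; On BeginPlay it registers itself by name in the BP_CheckPointManager's checkpoint map.
; When BP_My_Player overlaps its box, it sets the controller's last checkpoint and calls LoadPlayer.
; Despite its name, LoadPlayer saves: it flags respawn and copies checkpoint, mask and filter, weapon ammo, world-progress flags and quest items into BP_SaveGameInstance, the GameInstance.
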(event `self.ReceiveBeginPlay`
  (bind _returnvalue (`GameplayStatics.GetActorOfClass` "/Game/Blueprints/RespawnPlayer/BP_CheckPointManager.BP_CheckPointManager_C"))
  (`BlueprintMapLibrary.Map_Add` (`/Game/Blueprints/RespawnPlayer/BP_CheckPointManager.CheckPointMap` _returnvalue) (`self.NameSavePoint`) self))

(event `self.SavePointBox.OnComponentBeginOverlap`
  (params (OverlappedComponent :type "PrimitiveComponent Object Reference") (OtherActor :type "Actor Object Reference") (OtherComp :type "PrimitiveComponent Object Reference") (OtherBodyIndex :type Integer) (bFromSweep :type Boolean) (SweepResult :type "HitResult Structure (by ref)"))
  (cast `/Game/Blueprints/Player/BP_My_Player` OtherActor)
  (set `/Game/Blueprints/Player/BP_MainPlayerController.LastCheckPoint` (`self.NameSavePoint`) (`/Game/Blueprints/Player/FuctionLibrary/BFFL_CallPLayerController.CallMainPlayerController`))
  (`self.LoadPlayer`))

(event `LoadPlayer`
  (bind _myplayercharactere (`/Game/Blueprints/Player/FuctionLibrary/BFFL_CallPLayerController.CallMyPlayerCharactere`))
  (bind _myplayercharactere_2 (`/Game/Blueprints/Player/FuctionLibrary/BFFL_CallPLayerController.CallMyPlayerCharactere`))
  (bind _asbp_save_game_instance (cast `/Game/Blueprints/RespawnPlayer/BP_SaveGameInstance` (`GameplayStatics.GetGameInstance`) :!pure true))
  (bind _primaryweapon (`/Game/Blueprints/Player/BP_My_Player.PrimaryWeapon` (`/Game/Blueprints/Player/FuctionLibrary/BFFL_CallPLayerController.CallMyPlayerCharactere`)))
  (set `/Game/Blueprints/RespawnPlayer/BP_SaveGameInstance.Respawn` true _asbp_save_game_instance)
  (set `/Game/Blueprints/RespawnPlayer/BP_SaveGameInstance.LastCheckPointSave` (`/Game/Blueprints/Player/BP_MainPlayerController.LastCheckPoint` (`/Game/Blueprints/Player/FuctionLibrary/BFFL_CallPLayerController.CallMainPlayerController`)) _asbp_save_game_instance)
  (set `/Game/Blueprints/RespawnPlayer/BP_SaveGameInstance.SaveHaveMasque` (`/Game/Blueprints/Player/BP_My_Player.HaveMasque` _myplayercharactere) _asbp_save_game_instance)
  (set `/Game/Blueprints/RespawnPlayer/BP_SaveGameInstance.SaveFilterAmmout` (`/Game/Blueprints/Player/BP_My_Player.FilterAmount` _myplayercharactere) _asbp_save_game_instance)
  (set `/Game/Blueprints/RespawnPlayer/BP_SaveGameInstance.SaveActuelValueFiltre` (`/Game/Blueprints/Player/BP_My_Player.ActuelValueFiltre` _myplayercharactere) _asbp_save_game_instance)
  (set `/Game/Blueprints/RespawnPlayer/BP_SaveGameInstance.SaveCanEquipWeapon` (`/Game/Blueprints/Player/BP_My_Player.CanEquipWeapon` _myplayercharactere) _asbp_save_game_instance)
  (set `/Game/Blueprints/RespawnPlayer/BP_SaveGameInstance.SaveAmmocount` (`/Game/Weapon/Blueprints/BP_WeaponBase.Ammocount` _primaryweapon) _asbp_save_game_instance)
  (set `/Game/Blueprints/RespawnPlayer/BP_SaveGameInstance.SaveMaxAmmo` (`/Game/Weapon/Blueprints/BP_WeaponBase.MaxAmmo` _primaryweapon) _asbp_save_game_instance)
  (set `/Game/Blueprints/RespawnPlayer/BP_SaveGameInstance.SaveHaveKey` (`/Game/Blueprints/Player/BP_My_Player.HaveKey` _myplayercharactere_2) _asbp_save_game_instance)
  (set `/Game/Blueprints/RespawnPlayer/BP_SaveGameInstance.SavePontIsActive` (`/Game/Blueprints/Player/BP_My_Player.PontIsActive` _myplayercharactere_2) _asbp_save_game_instance)
  (set `/Game/Blueprints/RespawnPlayer/BP_SaveGameInstance.SaveActiveMeca` (`/Game/Blueprints/Player/BP_My_Player.ActiveMeca` _myplayercharactere_2) _asbp_save_game_instance)
  (set `/Game/Blueprints/RespawnPlayer/BP_SaveGameInstance.SaveDynamitePosee` (`/Game/Blueprints/Player/BP_My_Player.DynamitePosee` _myplayercharactere_2) _asbp_save_game_instance)
  (set `/Game/Blueprints/RespawnPlayer/BP_SaveGameInstance.SaveNomQuestItem1` (`/Game/Blueprints/Player/BP_My_Player.NomQuestItem1` _myplayercharactere_2) _asbp_save_game_instance)
  (set `/Game/Blueprints/RespawnPlayer/BP_SaveGameInstance.SaveNomQuestItem2` (`/Game/Blueprints/Player/BP_My_Player.NomQuestItem2` _myplayercharactere_2) _asbp_save_game_instance)
  (set `/Game/Blueprints/RespawnPlayer/BP_SaveGameInstance.SaveNbrQuestItems` (`/Game/Blueprints/Player/BP_My_Player.QuestItems` _myplayercharactere_2) _asbp_save_game_instance))

(fn `UserConstructionScript`)