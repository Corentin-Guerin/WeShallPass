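; BPC_SoundManager is a component that plays and stops one attached sound at a time.
; PlaySound spawns the given sound attached to the component and stores the audio component, ignoring calls while the SoundPlayed flag is set; its Emetteur input is unused.
; StopSound alone clears that flag, then stops and destroys the stored audio component, so a sound ending naturally still blocks new playback.
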(event `StopSound`
  (if (`self.SoundPlayed`)
    (set `self.SoundPlayed` false)
    (bind _audiocomponent (`self.AudioComponent`)
      (:`then`
        (`AudioComponent.Stop` _audiocomponent)
        (`self.K2_DestroyComponent` _audiocomponent))
      (:`else`))))

(event `PlaySound`
  (params (SoundToPlay :type "SoundBase Object Reference") (Emetteur :type "Vector Structure"))
  (if (not (`self.SoundPlayed`))
    (bind _returnvalue (`GameplayStatics.SpawnSoundAttached` SoundToPlay self "None" (0.0 0.0 0.0) (struct) "KeepRelativeOffset" false 1.0 1.0 0.0 null null))
    (set `self.AudioComponent` _returnvalue)
    (set `self.SoundPlayed` true)))