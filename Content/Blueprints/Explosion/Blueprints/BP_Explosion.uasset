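; BP_Explosion is an explosion actor whose Explosion event detonates it once, guarded by the IsExplos flag.
; After a short delay it fires a radial force impulse, activates its particle system and plays a sound through SoundManager.
; It spawns a scaled explosion emitter at the billboard's location and a steam emitter with no location set, then destroys itself after a further delay.
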(event `Explosion`
  (bind _soundmanager (`self.SoundManager`))
  (if (not (`self.IsExplos`))
    (`KismetSystemLibrary.Delay` 1.0)
    (`|ExecutionSequence`
      (:`then_0`
        (set `self.IsExplos` true))
      (:`then_1`
        (`RadialForceComponent.FireImpulse` (`self.RadialForce`)))
      (:`then_2`
        (`ActorComponent.Activate` (`self.ParticleSystem`) false)
        (`/Game/Blueprints/Sounds/BPC_SoundManager.PlaySound` _soundmanager (`self.ExplosionSound`) (`SceneComponent.K2_GetComponentLocation` _soundmanager)))
      (:`then_3`
        (`GameplayStatics.SpawnEmitterAtLocation` "/Game/StarterContent/Particles/P_Explosion.P_Explosion" (`SceneComponent.K2_GetComponentLocation` (`self.Billboard`)) (struct) (10.0 10.0 10.0))
        (`GameplayStatics.SpawnEmitterAtLocation` "/Game/StarterContent/Particles/P_Steam_Lit.P_Steam_Lit" (0.0 0.0 0.0) (struct) (10.0 10.0 10.0))
        (`KismetSystemLibrary.Delay` 5.0)
        (`self.K2_DestroyActor`)))))

(fn `UserConstructionScript`)