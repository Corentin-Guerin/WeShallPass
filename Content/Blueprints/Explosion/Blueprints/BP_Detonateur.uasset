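; BP_Detonateur is a one-time detonator that sets off an explosion when the player enters its trigger box.
; On overlap, if the player's ActiveMeca flag is still false, it sets the flag and calls Explosion on its Explosion reference.
; On BeginPlay it calls the same explosion if the save game instance's SaveActiveMeca flag is set, replaying the triggered state.
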(event `self.ReceiveBeginPlay`
  (if (`/Game/Blueprints/RespawnPlayer/BP_SaveGameInstance.SaveActiveMeca` (cast `/Game/Blueprints/RespawnPlayer/BP_SaveGameInstance` (`GameplayStatics.GetGameInstance`) :!pure true))
    (`/Game/Blueprints/Explosion/Blueprints/BP_Explosion.Explosion` (`self.Explosion`) :!label _label)))

(event `self.Triggerbox.OnComponentBeginOverlap`
  (params (OverlappedComponent :type "PrimitiveComponent Object Reference") (OtherActor :type "Actor Object Reference") (OtherComp :type "PrimitiveComponent Object Reference") (OtherBodyIndex :type Integer) (bFromSweep :type Boolean) (SweepResult :type "HitResult Structure (by ref)"))
  (bind _myplayercharactere (`/Game/Blueprints/Player/FuctionLibrary/BFFL_CallPLayerController.CallMyPlayerCharactere`))
  (cast `/Game/Blueprints/Player/BP_My_Player` OtherActor)
  (if (not (`/Game/Blueprints/Player/BP_My_Player.ActiveMeca` _myplayercharactere))
    (set `/Game/Blueprints/Player/BP_My_Player.ActiveMeca` true _myplayercharactere)
    (goto _label)))

(fn `UserConstructionScript`)