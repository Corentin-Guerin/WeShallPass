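; BP_QuestItem is an interactable quest pickup, apparently dynamite, that counts toward the player's quest items.
; On BeginPlay it sets up BPCInteractable and destroys itself if its name matches either quest item saved in the game instance.
; Interacting stores its name in one of two player slots, chosen by comparison with NomReference, and increments QuestItems.
; The pickup then destroys itself, shows WBP_Dynamite and plays a sound that differs for the first item.
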(event `self.ReceiveBeginPlay`
  (bind _bp_c_interactable (`self.BP_C_Interactable`))
  (set `/Game/Blueprints/Intercatible/BP_C_Interactable.NameItem` (`self.Name`) _bp_c_interactable)
  (set `/Game/Blueprints/Intercatible/BP_C_Interactable.WhichInterface` 0 _bp_c_interactable)
  (if (`KismetTextLibrary.EqualEqual_TextText` (`/Game/Blueprints/RespawnPlayer/BP_SaveGameInstance.SaveNomQuestItem1` (cast `/Game/Blueprints/RespawnPlayer/BP_SaveGameInstance` (`GameplayStatics.GetGameInstance`) :!pure true)) (`self.NomQuestItem`))
    (`self.K2_DestroyActor` :!label _label)
    (elif (`KismetTextLibrary.EqualEqual_TextText` (`/Game/Blueprints/RespawnPlayer/BP_SaveGameInstance.SaveNomQuestItem2` (cast `/Game/Blueprints/RespawnPlayer/BP_SaveGameInstance` (`GameplayStatics.GetGameInstance`) :!pure true)) (`self.NomQuestItem`))
      (goto _label))))

(event `self.BP_C_Interactable.Interact`
  (params (Player :type "/Game/Blueprints/Player/BP_My_Player Object Reference"))
  (if (`KismetTextLibrary.EqualEqual_TextText` (`self.NomQuestItem`) (`self.NomReference`))
    (set `/Game/Blueprints/Player/BP_My_Player.NomQuestItem1` (`self.NomQuestItem`) (`/Game/Blueprints/Player/FuctionLibrary/BFFL_CallPLayerController.CallMyPlayerCharactere`))
    (else
      (set `/Game/Blueprints/Player/BP_My_Player.NomQuestItem2` (`self.NomQuestItem`) (`/Game/Blueprints/Player/FuctionLibrary/BFFL_CallPLayerController.CallMyPlayerCharactere`))))
  (`/Game/Blueprints/Intercatible/BP_C_Interactable.DestroyInterface` (`self.BP_C_Interactable`))
  (set `/Game/Blueprints/Player/BP_My_Player.QuestItems` (+ (`/Game/Blueprints/Player/BP_My_Player.QuestItems` Player) 1) Player)
  (`self.K2_DestroyActor`)
  (bind _returnvalue (`|CreateWidget` "/Game/UI/InGame/WBP_Dynamite.WBP_Dynamite_C"))
  (`UserWidget.AddToViewport` _returnvalue 0)
  (if (== (`/Game/Blueprints/Player/BP_My_Player.QuestItems` (`/Game/Blueprints/Player/FuctionLibrary/BFFL_CallPLayerController.CallMyPlayerCharactere`)) 1)
    (`GameplayStatics.PlaySound2D` "/Game/Sounds/Dialogues/Bruts/DynamiteRené1.DynamiteRené1" 1.0 1.0 0.0 null null)
    (else
      (`GameplayStatics.PlaySound2D` "/Game/Sounds/Dialogues/Bruts/DynamiteRené2.DynamiteRené2" 1.0 1.0 0.0 null null))))

(fn `UserConstructionScript`)