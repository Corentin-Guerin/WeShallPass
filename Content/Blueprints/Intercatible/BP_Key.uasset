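; BP_Key is an interactable key pickup that grants the player a key.
; On BeginPlay it sets up its interactable component's item name and interface type, then destroys itself if the player character already has the key.
; Interacting through the BP_C_Interactable event removes the component's interface, sets HaveKey on the player, destroys the actor and plays a 2D pickup sound.
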(event `self.ReceiveBeginPlay`
  (bind _bp_c_interactable (`self.BP_C_Interactable`))
  (set `/Game/Blueprints/Intercatible/BP_C_Interactable.NameItem` (`self.Name`) _bp_c_interactable)
  (set `/Game/Blueprints/Intercatible/BP_C_Interactable.WhichInterface` 0 _bp_c_interactable)
  (if (`/Game/Blueprints/Player/BP_My_Player.HaveKey` (`/Game/Blueprints/Player/FuctionLibrary/BFFL_CallPLayerController.CallMyPlayerCharactere`))
    (`self.K2_DestroyActor`)))

(event `self.BP_C_Interactable.Interact`
  (params (Player :type "/Game/Blueprints/Player/BP_My_Player Object Reference"))
  (`/Game/Blueprints/Intercatible/BP_C_Interactable.DestroyInterface` (`self.BP_C_Interactable`))
  (set `/Game/Blueprints/Player/BP_My_Player.HaveKey` true Player)
  (`self.K2_DestroyActor`)
  (`GameplayStatics.PlaySound2D` "/Game/Sounds/Dialogues/Bruts/clé.clé" 1.0 1.0 0.0 null null))

(fn `UserConstructionScript`)