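; BP_CartoucheMasque is an interactable mask filter cartridge pickup.
; On interact it adds one to the player's FilterAmount and destroys itself, or shows WBP_Error if the count is already at the limit of three.
; BPCInteractable holds its display name and interface type, and removes that interface on pickup.
; Player overlap turns on a custom depth stencil highlight, cleared after a short delay or when the overlap ends.
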(event `self.ReceiveBeginPlay`
  (bind _bp_c_interactable (`self.BP_C_Interactable`))
  (set `/Game/Blueprints/Intercatible/BP_C_Interactable.NameItem` (`self.Name`) _bp_c_interactable)
  (set `/Game/Blueprints/Intercatible/BP_C_Interactable.WhichInterface` 0 _bp_c_interactable))

(event `self.BP_C_Interactable.Interact`
  (params (Player :type "/Game/Blueprints/Player/BP_My_Player Object Reference"))
  (if (< (`/Game/Blueprints/Player/BP_My_Player.FilterAmount` Player) 3)
    (`/Game/Blueprints/Intercatible/BP_C_Interactable.DestroyInterface` (`self.BP_C_Interactable`))
    (set `/Game/Blueprints/Player/BP_My_Player.FilterAmount` (+ (`/Game/Blueprints/Player/BP_My_Player.FilterAmount` Player) 1) Player)
    (`self.K2_DestroyActor`)
    (else
      (bind _returnvalue (`|CreateWidget` "/Game/UI/InGame/WBP_Error.WBP_Error_C"))
      (`UserWidget.AddToViewport` _returnvalue 0))))

(event `self.ReceiveActorBeginOverlap`
  (params (OtherActor :type "Actor Object Reference"))
  (bind _bp_c_interactable (`self.BP_C_Interactable`))
  (cast `/Game/Blueprints/Player/BP_My_Player` OtherActor)
  (`PrimitiveComponent.SetRenderCustomDepth` _bp_c_interactable true)
  (`PrimitiveComponent.SetCustomDepthStencilValue` _bp_c_interactable 2)
  (`KismetSystemLibrary.Delay` 3.0)
  (`PrimitiveComponent.SetRenderCustomDepth` _bp_c_interactable false :!label _label)
  (`PrimitiveComponent.SetCustomDepthStencilValue` _bp_c_interactable 0))

(event `self.ReceiveActorEndOverlap`
  (params (OtherActor :type "Actor Object Reference"))
  (cast `/Game/Blueprints/Player/BP_My_Player` OtherActor)
  (goto _label))

(fn `UserConstructionScript`)