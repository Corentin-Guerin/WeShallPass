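; Interactable Blueprint that shows and hides an on-screen interaction prompt as feedback for whether it can be interacted with.
; CanInteractFeedBack creates a WBP_TexteInteraction widget, stores it and adds it to the viewport.
; CantInteractFeedBack removes that stored widget through DestroyInterface.
; An unconnected material swap to M_Alight and back remains in the graph but never runs.
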(event `CanInteractFeedBack`
  (bind _returnvalue (`|CreateWidget` "/Game/UI/InGame/WBP_TexteInteraction.WBP_TexteInteraction_C"))
  (bind _output_get (set `self.InterfaceInteract` _returnvalue))
  (`UserWidget.AddToViewport` _output_get 0))

(event `CantInteractFeedBack`
  (`self.DestroyInterface`))

(fn `DestroyInterface`
  (`Widget.RemoveFromParent` (`self.InterfaceInteract`)))