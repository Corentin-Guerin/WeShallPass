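; BP_Detonateur is an interactable detonator that blows up the bridge (Pont) once dynamite has been placed.
; On BeginPlay it passes its name and interface type to its BPCInteractable component.
; Interacting removes that interface and, if the referenced dynamite is placed, blends the view to CinematiqueExplosion with input disabled.
; Timed delays trigger Kaboom on the bridge, then return view and input to the player.
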(event `self.ReceiveBeginPlay`
  (bind _bp_c_interactable (`self.BP_C_Interactable`))
  (set `/Game/Blueprints/Intercatible/BP_C_Interactable.NameItem` (`self.Name`) _bp_c_interactable)
  (set `/Game/Blueprints/Intercatible/BP_C_Interactable.WhichInterface` 2 _bp_c_interactable))

(event `self.BP_C_Interactable.Interact`
  (params (Player :type "/Game/Blueprints/Player/BP_My_Player Object Reference"))
  (bind _returnvalue (`GameplayStatics.GetPlayerController` 0))
  (bind _returnvalue_2 (`GameplayStatics.GetPlayerCharacter` 0))
  (`/Game/Blueprints/Intercatible/BP_C_Interactable.DestroyInterface` (`self.BP_C_Interactable`))
  (if (`/Game/Blueprints/Intercatible/BP_DynamitePose.DynamitePosée` (`self.Dynamiteposée`))
    (`PlayerController.SetViewTargetWithBlend` _returnvalue (`self.CinematiqueExplosion`) 0.0 "VTBlend_Linear" 0.0 false)
    (`self.DisableInput` _returnvalue_2 _returnvalue)
    (`KismetSystemLibrary.Delay` 0.5)
    (`/Game/Blueprints/Pont/BP_Pont.Kaboom` (`self.Pont`))
    (`KismetSystemLibrary.Delay` 3.9)
    (`PlayerController.SetViewTargetWithBlend` _returnvalue _returnvalue_2 0.0 "VTBlend_Linear" 0.0 false)
    (`self.EnableInput` _returnvalue_2 _returnvalue)))

(fn `UserConstructionScript`)