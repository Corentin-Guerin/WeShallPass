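; Interactable ammo box that refills the player's primary weapon.
; On BeginPlay it passes its name and interface type to its BPCInteractable component.
; The Interact event sets the primary weapon's Ammocount to its AmmoChargeur value on player 0's character.
; Any actor overlap turns on a custom depth stencil highlight, cleared after a short delay or when the overlap ends.
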(event `self.ReceiveBeginPlay`
  (bind _bp_c_interactable (`self.BP_C_Interactable`))
  (set `/Game/Blueprints/Intercatible/BP_C_Interactable.NameItem` (`self.Name`) _bp_c_interactable)
  (set `/Game/Blueprints/Intercatible/BP_C_Interactable.WhichInterface` 2 _bp_c_interactable))

(event `self.BP_C_Interactable.Interact`
  (params (Player :type "/Game/Blueprints/Player/BP_My_Player Object Reference"))
  (bind _primaryweapon (`/Game/Blueprints/Player/BP_My_Player.PrimaryWeapon` (cast `/Game/Blueprints/Player/BP_My_Player` (`GameplayStatics.GetPlayerCharacter` 0) :!pure true)))
  (set `/Game/Weapon/Blueprints/BP_WeaponBase.Ammocount` (`/Game/Weapon/Blueprints/BP_WeaponBase.AmmoChargeur` _primaryweapon) _primaryweapon))

(event `self.ReceiveActorBeginOverlap`
  (params (OtherActor :type "Actor Object Reference"))
  (bind _bp_c_interactable (`self.BP_C_Interactable`))
  (`PrimitiveComponent.SetRenderCustomDepth` _bp_c_interactable true)
  (`PrimitiveComponent.SetCustomDepthStencilValue` _bp_c_interactable 2)
  (`KismetSystemLibrary.Delay` 3.0)
  (`PrimitiveComponent.SetRenderCustomDepth` _bp_c_interactable false :!label _label)
  (`PrimitiveComponent.SetCustomDepthStencilValue` _bp_c_interactable 0))

(event `self.ReceiveActorEndOverlap`
  (params (OtherActor :type "Actor Object Reference"))
  (goto _label))

(fn `UserConstructionScript`)