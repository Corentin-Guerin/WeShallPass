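; LockDoor is an interactable door held by a padlock that the player can shoot off.
; A BP_TracerBullet overlapping the padlock (Cadena) destroys it and flags the door as unlocked.
; Interacting with Porte, which receives the item name and interface type at BeginPlay, then plays a timeline that sets the pivot's world yaw to swing the door open, but only once the padlock is gone.
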(event `self.ReceiveBeginPlay`
  (bind _porte (`self.Porte`))
  (set `/Game/Blueprints/Intercatible/BP_C_Interactable.NameItem` (`self.Name`) _porte)
  (set `/Game/Blueprints/Intercatible/BP_C_Interactable.WhichInterface` 2 _porte))

(event `self.Cadena.OnComponentBeginOverlap`
  (params (OverlappedComponent :type "PrimitiveComponent Object Reference") (OtherActor :type "Actor Object Reference") (OtherComp :type "PrimitiveComponent Object Reference") (OtherBodyIndex :type Integer) (bFromSweep :type Boolean) (SweepResult :type "HitResult Structure (by ref)"))
  (cast `/Game/Weapon/Blueprints/BP_TracerBullet` OtherActor)
  (`ActorComponent.K2_DestroyComponent` (`self.Cadena`))
  (set `self.CadenaIsDestroy` true))

(event `self.Porte.Interact`
  (params (Player :type "/Game/Blueprints/Player/BP_My_Player Object Reference"))
  (if (`self.CadenaIsDestroy`)
    (bind (_direction _newtrack_0) (`Timeline|Timeline_0`)
      (:`Update`
        (`SceneComponent.K2_SetWorldRotation` (`self.Pivot`) (`KismetMathLibrary.MakeRotator` 0.0 0.0 _newtrack_0) false false)))))

(fn `UserConstructionScript`)