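; Interactable dynamite placement spot that the player completes once they hold at least two quest items.
; On BeginPlay it passes its name and interface type to its BPCInteractable.
; On interaction it removes the interface, then, if the quest item count suffices, swaps in the dynamite, rod and wire materials and flags the dynamite as placed.
; The interface is removed even when the item check fails.
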(event `self.ReceiveBeginPlay`
  (bind _bp_c_interactable (`self.BP_C_Interactable`))
  (set `/Game/Blueprints/Intercatible/BP_C_Interactable.NameItem` (`self.Name`) _bp_c_interactable)
  (set `/Game/Blueprints/Intercatible/BP_C_Interactable.WhichInterface` 1 _bp_c_interactable))

(event `self.BP_C_Interactable.Interact`
  (params (Player :type "/Game/Blueprints/Player/BP_My_Player Object Reference"))
  (bind _bp_c_interactable (`self.BP_C_Interactable`))
  (`/Game/Blueprints/Intercatible/BP_C_Interactable.DestroyInterface` (`self.BP_C_Interactable`))
  (if (>= (`/Game/Blueprints/Player/BP_My_Player.QuestItems` Player) 2)
    (`PrimitiveComponent.SetMaterial` _bp_c_interactable 0 "/Game/Meshes/Interractible/Dynamites/Textures/Baton/M_Dynamites.M_Dynamites")
    (`PrimitiveComponent.SetMaterial` _bp_c_interactable 1 "/Game/Meshes/Interractible/Dynamites/Textures/Tige/M_Tige.M_Tige")
    (`PrimitiveComponent.SetMaterial` _bp_c_interactable 2 "/Game/Meshes/Interractible/Dynamites/Textures/Fil/M_Fil.M_Fil")
    (`PrimitiveComponent.SetMaterial` _bp_c_interactable 3 "/Game/Meshes/Interractible/Dynamites/Textures/Fil/M_Fil.M_Fil")
    (set `self.DynamitePosée` true)))

(fn `UserConstructionScript`)