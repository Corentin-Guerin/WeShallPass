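; Gas mask pickup that the player collects through the interactable component's Interact event.
; Interacting sets HaveMasque on the character, calls BindEventToMasqueGaz on the main controller, destroys the actor, adds mask and tutorial widgets, and plays a sound.
; Overlap turns on custom depth and stencil highlighting, cleared after a short delay or when overlap ends.
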(event `self.ReceiveBeginPlay`
  (bind _bp_c_interactable (`self.BP_C_Interactable`))
  (set `/Game/Blueprints/Intercatible/BP_C_Interactable.NameItem` (`self.Name`) _bp_c_interactable)
  (set `/Game/Blueprints/Intercatible/BP_C_Interactable.WhichInterface` 0 _bp_c_interactable))

(event `self.BP_C_Interactable.Interact`
  (params (Player :type "/Game/Blueprints/Player/BP_My_Player Object Reference"))
  (`/Game/Blueprints/Intercatible/BP_C_Interactable.DestroyInterface` (`self.BP_C_Interactable`))
  (set `/Game/Blueprints/Player/BP_My_Player.HaveMasque` true (`/Game/Blueprints/Player/FuctionLibrary/BFFL_CallPLayerController.CallMyPlayerCharactere`))
  (add `/Game/Blueprints/Player/BP_MainPlayerController.MasqueGaz` (`/Game/Blueprints/Player/FuctionLibrary/BFFL_CallPLayerController.CallMainPlayerController`) (`|CreateDelegate` Player :!event `EquipeMasqueAGaz`))
  (`self.K2_DestroyActor`)
  (bind _returnvalue (`|CreateWidget` "/Game/UI/InGame/WBP_Masque.WBP_Masque_C"))
  (`UserWidget.AddToViewport` _returnvalue 0)
  (bind _returnvalue_2 (`|CreateWidget` "/Game/UI/InGame/Tutos/WBP_Tuto_Masque.WBP_Tuto_Masque_C"))
  (`UserWidget.AddToViewport` _returnvalue_2 0)
  (`GameplayStatics.PlaySound2D` "/Game/Sounds/Dialogues/Bruts/Gaz.Gaz" 1.0 1.0 0.0 null null))

(event `self.ReceiveActorBeginOverlap`
  (params (OtherActor :type "Actor Object Reference"))
  (bind _bp_c_interactable (`self.BP_C_Interactable`))
  (`PrimitiveComponent.SetRenderCustomDepth` _bp_c_interactable true)
  (`PrimitiveComponent.SetCustomDepthStencilValue` _bp_c_interactable 2)
  (`KismetSystemLibrary.Delay` 3.0)
  (`PrimitiveComponent.SetRenderCustomDepth` _bp_c_interactable false :!label _label)
  (`PrimitiveComponent.SetCustomDepthStencilValue` _bp_c_interactable 0))

(event `self.ReceiveActorEndOverlap`
  (params (OtherActor :type "Actor Object Reference"))
  (goto _label))

(fn `UserConstructionScript`)