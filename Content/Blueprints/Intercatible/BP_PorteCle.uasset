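; BP_PorteCle is an interactable locked door that opens only when the interacting player has a key.
; On BeginPlay it passes its name and interface type to the BPCInteractable component.
; A successful interaction destroys the component's interface, then plays a timeline that drives the world yaw of BPCInteractable, with pitch and roll held at zero.
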(event `self.ReceiveBeginPlay`
  (bind _bp_c_interactable (`self.BP_C_Interactable`))
  (set `/Game/Blueprints/Intercatible/BP_C_Interactable.NameItem` (`self.Name`) _bp_c_interactable)
  (set `/Game/Blueprints/Intercatible/BP_C_Interactable.WhichInterface` 2 _bp_c_interactable))

(event `self.BP_C_Interactable.Interact`
  (params (Player :type "/Game/Blueprints/Player/BP_My_Player Object Reference"))
  (if (`/Game/Blueprints/Player/BP_My_Player.HaveKey` Player)
    (`/Game/Blueprints/Intercatible/BP_C_Interactable.DestroyInterface` (`self.BP_C_Interactable`))
    (bind (_direction _newtrack_0) (`Timeline|Timeline_0`)
      (:`Update`
        (`SceneComponent.K2_SetWorldRotation` (`self.BP_C_Interactable`) (`KismetMathLibrary.MakeRotator` 0.0 0.0 _newtrack_0) false false)))))

(fn `UserConstructionScript`)