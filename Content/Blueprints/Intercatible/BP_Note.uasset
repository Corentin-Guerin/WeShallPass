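; BP_Note is an interactable note actor that shows a notes screen when the player uses it.
; On BeginPlay it passes its Name to the interactable component as the item name.
; On Interact it removes the component's interface, creates and shows a WPB_Notes widget, pauses the game and shows the mouse cursor.
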(event `self.ReceiveBeginPlay`
  (set `/Game/Blueprints/Intercatible/BP_C_Interactable.NameItem` (`self.Name`) (`self.BP_C_Interactable`)))

(event `self.BP_C_Interactable.Interact`
  (params (Player :type "/Game/Blueprints/Player/BP_My_Player Object Reference"))
  (`/Game/Blueprints/Intercatible/BP_C_Interactable.DestroyInterface` (`self.BP_C_Interactable`))
  (bind _returnvalue (`|CreateWidget` "/Game/UI/InGame/WPB_Notes.WPB_Notes_C"))
  (bind _output_get (set `self.Notes` _returnvalue))
  (`UserWidget.AddToViewport` _output_get 0)
  (`GameplayStatics.SetGamePaused` true)
  (set `PlayerController.bShowMouseCursor` true (`GameplayStatics.GetPlayerController` 0)))

(fn `UserConstructionScript`)