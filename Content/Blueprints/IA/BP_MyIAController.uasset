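; AI controller for the "Meca" enemy, running BT_MecaBT on the BB_MyMeca blackboard.
; On BeginPlay it registers with every BP_IAISubscibable actor and stores the player reference, stage (Etape) flags and random patrol targets, one general and one per stage, in the blackboard.
; Each Tick it copies the player character's chase and discovered flags into the IsChase and IsAgro keys for the behavior tree.
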(event `self.ReceiveBeginPlay`
  (`|ExecutionSequence`
    (:`then_0`
      (`self.SubscribeAllSubscribable`))
    (:`then_1`
      (bind _blackboardcomponent (`self.UseBlackboard` "/Game/Blueprints/IA/BB_MyMeca.BB_MyMeca"))
      (bind _output_get (set `self.Blackboard Component` _blackboardcomponent))
      (`self.ResetBool`)
      (`BlackboardComponent.SetValueAsObject` _output_get "PlayerRef" (`GameplayStatics.GetPlayerCharacter` 0))
      (`self.SetRandomTargetPoint`)
      (`self.SetRandomTargetPointEtape1`)
      (`self.SetRandomTargetPointEtape2`)
      (`self.SetRandomTargetPointEtape3`)
      (`self.SetRandomTargetPointEtape4`)
      (`self.SetRandomTargetPointEtape5`)
      (`self.SwitchEtape`)
      (`self.RunBehaviorTree` "/Game/Blueprints/IA/BT_MecaBT.BT_MecaBT"))))

(event `self.ReceiveTick`
  (params (DeltaSeconds :type "Float (single-precision)"))
  (`self.ResetBool`))

(event `SwitchEtape`
  (`BlackboardComponent.SetValueAsBool` (`self.Blackboard Component`) "Etape1" (`self.Etape1`))
  (`BlackboardComponent.SetValueAsBool` (`self.Blackboard Component`) "Etape2" (`self.Etape2`))
  (`BlackboardComponent.SetValueAsBool` (`self.Blackboard Component`) "Etape3" (`self.Etape3`))
  (`BlackboardComponent.SetValueAsBool` (`self.Blackboard Component`) "Etape4" (`self.Etape4`))
  (`BlackboardComponent.SetValueAsBool` (`self.Blackboard Component`) "Etape5" (`self.Etape5`)))

(event `ResetBool`
  (`BlackboardComponent.SetValueAsBool` (`self.Blackboard Component`) "IsChase" (`/Game/Blueprints/Player/BP_My_Player.IsChase` (`/Game/Blueprints/Player/FuctionLibrary/BFFL_CallPLayerController.CallMyPlayerCharactere`)))
  (`BlackboardComponent.SetValueAsBool` (`self.Blackboard Component`) "IsAgro" (`/Game/Blueprints/Player/BP_My_Player.IsDiscover` (`/Game/Blueprints/Player/FuctionLibrary/BFFL_CallPLayerController.CallMyPlayerCharactere`))))

(fn `SetRandomTargetPoint`
  (bind _targetpoints (`self.TargetPoints`))
  (`BlackboardComponent.SetValueAsObject` (`self.Blackboard Component`) "Target" (`|GetArrayItem` _targetpoints (`KismetMathLibrary.RandomIntegerInRange` 0 (- (`KismetArrayLibrary.Array_Length` _targetpoints) 1)))))

(fn `SetRandomTargetPointEtape1`
  (bind _targetspointsetape1 (`self.TargetsPointsEtape1`))
  (`BlackboardComponent.SetValueAsObject` (`self.Blackboard Component`) "TargetEtape1" (`|GetArrayItem` _targetspointsetape1 (`KismetMathLibrary.RandomIntegerInRange` 0 (- (`KismetArrayLibrary.Array_Length` _targetspointsetape1) 1)))))

(fn `SetRandomTargetPointEtape2`
  (bind _targetspointsetape2 (`self.TargetsPointsEtape2`))
  (`BlackboardComponent.SetValueAsObject` (`self.Blackboard Component`) "TargetEtape2" (`|GetArrayItem` _targetspointsetape2 (`KismetMathLibrary.RandomIntegerInRange` 0 (- (`KismetArrayLibrary.Array_Length` _targetspointsetape2) 1)))))

(fn `SetRandomTargetPointEtape3`
  (bind _targetspointsetape3 (`self.TargetsPointsEtape3`))
  (`BlackboardComponent.SetValueAsObject` (`self.Blackboard Component`) "TargetEtape3" (`|GetArrayItem` _targetspointsetape3 (`KismetMathLibrary.RandomIntegerInRange` 0 (- (`KismetArrayLibrary.Array_Length` _targetspointsetape3) 1)))))

(fn `SetRandomTargetPointEtape4`
  (bind _targetspointsetape4 (`self.TargetsPointsEtape4`))
  (`BlackboardComponent.SetValueAsObject` (`self.Blackboard Component`) "TargetEtape4" (`|GetArrayItem` _targetspointsetape4 (`KismetMathLibrary.RandomIntegerInRange` 0 (- (`KismetArrayLibrary.Array_Length` _targetspointsetape4) 1)))))

(fn `SetRandomTargetPointEtape5`
  (bind _targetspointsetape5 (`self.TargetsPointsEtape5`))
  (`BlackboardComponent.SetValueAsObject` (`self.Blackboard Component`) "TargetEtape5" (`|GetArrayItem` _targetspointsetape5 (`KismetMathLibrary.RandomIntegerInRange` 0 (- (`KismetArrayLibrary.Array_Length` _targetspointsetape5) 1)))))

(fn `SubscribeAllSubscribable`
  (bind _outactors (`GameplayStatics.GetAllActorsWithInterface` "/Game/Blueprints/Player/BP_IAISubscibable.BP_IAISubscibable_C"))
  (for _array_element _outactors
    (message `/Game/Blueprints/Player/BP_IAISubscibable.Subscribe` _array_element self)))

(fn `UserConstructionScript`)