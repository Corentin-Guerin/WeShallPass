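; Mech AI actor with two lamps that signal whether the player has been detected.
; Each Tick reads the player's discovered and chase flags, switches light colors, plays a one-shot alert sound and aims both spotlights at the player.
; Otherwise it restores the undetected color and starting rotations and resets the sound.
; A tracer bullet overlapping either lamp's sphere hides that lamp and flags it destroyed for a few seconds.
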(event `self.ReceiveTick`
  (params (DeltaSeconds :type "Float (single-precision)"))
  (bind _myplayercharactere (`/Game/Blueprints/Player/FuctionLibrary/BFFL_CallPLayerController.CallMyPlayerCharactere`))
  (if (or (`/Game/Blueprints/Player/BP_My_Player.IsDiscover` _myplayercharactere) (`/Game/Blueprints/Player/BP_My_Player.IsChase` _myplayercharactere))
    (`|ExecutionSequence`
      (:`then_0`
        (`LightComponent.SetLightColor` (`self.SpotLight`) (`self.DetectColor`) true)
        (`LightComponent.SetLightColor` (`self.PointLight`) (`self.DetectColor`) true)
        (`LightComponent.SetLightColor` (`self.SpotLight1`) (`self.DetectColor`) true)
        (`LightComponent.SetLightColor` (`self.PointLight1`) (`self.DetectColor`) true)
        (`/Game/Blueprints/Sounds/BPC_SoundManager.PlaySoundOnce` (`self.BPC_SoundManager`) (`self.CriMeca`)))
      (:`then_1`
        (`SceneComponent.K2_SetWorldRotation` (`self.SpotLight`) (`KismetMathLibrary.FindLookAtRotation` (`SceneComponent.K2_GetComponentLocation` (`self.StaticMesh`)) (`SceneComponent.K2_GetComponentLocation` (`Character.CapsuleComponent` (`/Game/Blueprints/Player/FuctionLibrary/BFFL_CallPLayerController.CallMyPlayerCharactere`)))) true true)
        (`SceneComponent.K2_SetWorldRotation` (`self.SpotLight1`) (`KismetMathLibrary.FindLookAtRotation` (`SceneComponent.K2_GetComponentLocation` (`self.StaticMesh`)) (`SceneComponent.K2_GetComponentLocation` (`Character.CapsuleComponent` (`/Game/Blueprints/Player/FuctionLibrary/BFFL_CallPLayerController.CallMyPlayerCharactere`)))) true true)))
    (else
      (`LightComponent.SetLightColor` (`self.SpotLight`) (`self.UndetectColor`) true)
      (`LightComponent.SetLightColor` (`self.PointLight`) (`self.UndetectColor`) true)
      (`LightComponent.SetLightColor` (`self.SpotLight1`) (`self.UndetectColor`) true)
      (`LightComponent.SetLightColor` (`self.PointLight1`) (`self.UndetectColor`) true)
      (`SceneComponent.K2_SetWorldRotation` (`self.PointLight`) (`self.Default Spot Light Rot`) false false)
      (`SceneComponent.K2_SetWorldRotation` (`self.SpotLight`) (`self.Default Spot Light Rot`) false false)
      (`SceneComponent.K2_SetWorldRotation` (`self.PointLight1`) (`self.Default Spot Light1 Rot`) false false)
      (`SceneComponent.K2_SetWorldRotation` (`self.SpotLight1`) (`self.Default Spot Light1 Rot`) false false)
      (`/Game/Blueprints/Sounds/BPC_SoundManager.ResetSoundPlayed` (`self.BPC_SoundManager`)))))

(event `self.ReceiveBeginPlay`
  (set `self.Default Spot Light1 Rot` (`SceneComponent.K2_GetComponentRotation` (`self.PointLight1`)))
  (set `self.Default Spot Light Rot` (`SceneComponent.K2_GetComponentRotation` (`self.PointLight`))))

(event `self.Sphere.OnComponentBeginOverlap`
  (params (OverlappedComponent :type "PrimitiveComponent Object Reference") (OtherActor :type "Actor Object Reference") (OtherComp :type "PrimitiveComponent Object Reference") (OtherBodyIndex :type Integer) (bFromSweep :type Boolean) (SweepResult :type "HitResult Structure (by ref)"))
  (cast `/Game/Weapon/Blueprints/BP_TracerBullet` OtherActor)
  (`SceneComponent.SetVisibility` (`self.PointLight`) false false)
  (`SceneComponent.SetVisibility` (`self.SpotLight`) false false)
  (set `self.Spot1Destroy` true)
  (`KismetSystemLibrary.Delay` 5.0)
  (`SceneComponent.SetVisibility` (`self.PointLight`) true false)
  (`SceneComponent.SetVisibility` (`self.SpotLight`) true false)
  (set `self.Spot1Destroy` false))

(event `self.Sphere1.OnComponentBeginOverlap`
  (params (OverlappedComponent :type "PrimitiveComponent Object Reference") (OtherActor :type "Actor Object Reference") (OtherComp :type "PrimitiveComponent Object Reference") (OtherBodyIndex :type Integer) (bFromSweep :type Boolean) (SweepResult :type "HitResult Structure (by ref)"))
  (cast `/Game/Weapon/Blueprints/BP_TracerBullet` OtherActor)
  (`SceneComponent.SetVisibility` (`self.PointLight1`) false false)
  (`SceneComponent.SetVisibility` (`self.SpotLight1`) false false)
  (set `self.Spot2Destroy` true)
  (`KismetSystemLibrary.Delay` 5.0)
  (`SceneComponent.SetVisibility` (`self.PointLight1`) true false)
  (`SceneComponent.SetVisibility` (`self.SpotLight1`) true false)
  (set `self.Spot2Destroy` false))

(fn `UserConstructionScript`)