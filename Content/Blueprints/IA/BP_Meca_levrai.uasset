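; Enemy mecha that sweeps a searchlight for the player and kills on a gunshot hit or on contact during a chase.
; Cone overlap plus a line trace triggers detection, driving light color, aiming and delayed hitscan fire with random spread and tracers.
; Losing sight runs a Delay-based timer on Tick that clears the alert, while bullets temporarily knock out the spotlight.
; The player's IsChase flag switches it to flames, radial impulses and movement sound.
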(event `self.ReceiveTick`
  (params (DeltaSeconds :type "Float (single-precision)"))
  (bind _myplayercharactere (`/Game/Blueprints/Player/FuctionLibrary/BFFL_CallPLayerController.CallMyPlayerCharactere`))
  (bind _firesound1 (`self.fireSound1`))
  (`SkeletalMeshComponent.SetAnimInstanceClass` (`self.Mecha_Bas`) "/Game/Animation/Mecha/MechaBas_AnimeBP.MechaBas_AnimeBP_C")
  (if (`/Game/Blueprints/Player/BP_My_Player.IsChase` (`/Game/Blueprints/Player/FuctionLibrary/BFFL_CallPLayerController.CallMyPlayerCharactere`))
    (set `self.MecaChase` true)
    (`/Game/Blueprints/Sounds/BPC_SoundManager.StopSound` (`self.IdleSound`))
    (`/Game/Blueprints/Sounds/BPC_SoundManager.PlaySound` (`self.MoveSound`) (`self.Move`) (`self.K2_GetActorLocation`))
    (else
      (set `self.MecaChase` false)
      (`/Game/Blueprints/Sounds/BPC_SoundManager.StopSound` (`self.MoveSound`))
      (`/Game/Blueprints/Sounds/BPC_SoundManager.PlaySound` (`self.IdleSound`) (`self.Idle`) (`self.K2_GetActorLocation`))))
  (if (and (not (`/Game/Blueprints/Player/BP_My_Player.IsChase` _myplayercharactere)) (not (`/Game/Blueprints/Player/BP_My_Player.IsDiscover` _myplayercharactere)) (not (`self.IsTrigger`)))
    (`self.RotationSpot`)
    (if (not (`self.ResetCourse`))
      (`LightComponent.SetLightColor` (`self.PointLight`) (`self.DefaultColor`) true)
      (`LightComponent.SetLightColor` (`self.SpotLight`) (`self.DefaultColor`) true)
      (`SceneComponent.K2_SetRelativeRotation` (`self.ProjecteurDroit`) (`self.DefautRotProjDroite`) false false)
      (`SceneComponent.K2_SetRelativeRotation` (`self.PivotBrasDroit`) (`self.DefautRotBrasDroite`) false false)
      (`SceneComponent.K2_SetRelativeRotation` (`self.PivotHaut`) (`self.DefautRotMeca`) false false)
      (set `self.ResetCourse` true)
      (set `self.OpenFire` false)
      (`/Game/Blueprints/Sounds/BPC_SoundManager.StopSound` (`self.CriSound`)))
    (else
      (set `self.ResetCourse` false)
      (`|ExecutionSequence`
        (:`then_0`
          (`self.RotationMechaWhenFocus`))
        (:`then_1`
          (`LightComponent.SetLightColor` (`self.SpotLight`) (`self.DetectColor`) true)
          (`LightComponent.SetLightColor` (`self.PointLight`) (`self.DetectColor`) true))
        (:`then_2`
          (bind _hitactor (`self.Detectiondujoueur` (`self.SpotLight`)))
          (cast `/Game/Blueprints/Player/BP_My_Player` _hitactor
            (:`then`
              (set `self.Joueurcacher` false))
            (:`CastFailed`
              (set `self.Joueurcacher` true)))
          (if (`self.Joueurcacher`)
            (`KismetSystemLibrary.Delay` 1.0)
            (set `self.Timerjoueurcacher` (+ (`self.Timerjoueurcacher`) 1.0))
            (if (== (`self.Timerjoueurcacher`) 5.0)
              (set `self.Timerjoueurcacher` 0.0)
              (set `/Game/Blueprints/Player/BP_My_Player.IsDiscover` false (`/Game/Blueprints/Player/FuctionLibrary/BFFL_CallPLayerController.CallMyPlayerCharactere`))
              (set `self.IsTrigger` false)
              (set `self.Joueurcacher` false))
            (else
              (set `self.Timerjoueurcacher` 0.0)
              (set `/Game/Blueprints/Player/BP_My_Player.IsDiscover` true (`/Game/Blueprints/Player/FuctionLibrary/BFFL_CallPLayerController.CallMyPlayerCharactere`))
              (set `self.IsTrigger` true))))
        (:`then_3`
          (if (or (`/Game/Blueprints/Player/BP_My_Player.IsChase` (`/Game/Blueprints/Player/FuctionLibrary/BFFL_CallPLayerController.CallMyPlayerCharactere`)) (`self.Spot1Destroy`))
            (set `self.OpenFire` false)
            (elif (`self.ActiveMeca`)
              (if (not (`self.OpenFire`))
                (`KismetSystemLibrary.Delay` 5.0)
                (set `self.OpenFire` true)
                (else
                  (`KismetSystemLibrary.Delay` 1.0)
                  (`self.ShootPlayerFocus`))))))
        (:`then_4`
          (if (`/Game/Blueprints/Player/BP_My_Player.IsChase` (`/Game/Blueprints/Player/FuctionLibrary/BFFL_CallPLayerController.CallMyPlayerCharactere`))
            (`RadialForceComponent.FireImpulse` (`self.RadialForce`))
            (`SceneComponent.SetVisibility` (`self.Feu1`) true false)
            (`SceneComponent.SetVisibility` (`self.Feu2`) true false)
            (`SceneComponent.SetVisibility` (`self.Feu3`) true false)
            (`/Game/Blueprints/Sounds/BPC_SoundManager.PlaySound` _firesound1 "/Game/Sounds/SCue_Firemeca.SCue_Firemeca" (`SceneComponent.K2_GetComponentLocation` _firesound1))))))))

(event `self.ReceiveBeginPlay`
  (bind _idlesound (`self.IdleSound`))
  (set `self.DefautRotProjDroite` (`SceneComponent.RelativeRotation` (`self.ProjecteurDroit`)))
  (set `self.DefautRotMeca` (`SceneComponent.RelativeRotation` (`self.PivotHaut`)))
  (set `self.DefautRotBrasDroite` (`SceneComponent.RelativeRotation` (`self.PivotBrasDroit`)))
  (`/Game/Blueprints/Sounds/BPC_SoundManager.PlaySound` _idlesound (`self.Idle`) (`SceneComponent.K2_GetComponentLocation` _idlesound))
  (`SceneComponent.SetVisibility` (`self.Feu1`) false false)
  (`SceneComponent.SetVisibility` (`self.Feu2`) false false)
  (`SceneComponent.SetVisibility` (`self.Feu3`) false false))

(event `self.ConeDroite.OnComponentBeginOverlap`
  (params (OverlappedComponent :type "PrimitiveComponent Object Reference") (OtherActor :type "Actor Object Reference") (OtherComp :type "PrimitiveComponent Object Reference") (OtherBodyIndex :type Integer) (bFromSweep :type Boolean) (SweepResult :type "HitResult Structure (by ref)"))
  (bind _crisound (`self.CriSound`))
  (cast `/Game/Blueprints/Player/BP_My_Player` OtherActor)
  (if (not (`self.Joueurcacher`))
    (bind _hitactor (`self.Detectiondujoueur` (`self.SpotLight`)))
    (cast `/Game/Blueprints/Player/BP_My_Player` _hitactor)
    (set `self.IsTrigger` true)
    (set `/Game/Blueprints/Player/BP_My_Player.IsDiscover` true (`/Game/Blueprints/Player/FuctionLibrary/BFFL_CallPLayerController.CallMyPlayerCharactere`))
    (`/Game/Blueprints/Sounds/BPC_SoundManager.PlaySound` _crisound (`self.Cri`) (`SceneComponent.K2_GetComponentLocation` _crisound))))

(event `self.Sphere.OnComponentBeginOverlap`
  (params (OverlappedComponent :type "PrimitiveComponent Object Reference") (OtherActor :type "Actor Object Reference") (OtherComp :type "PrimitiveComponent Object Reference") (OtherBodyIndex :type Integer) (bFromSweep :type Boolean) (SweepResult :type "HitResult Structure (by ref)"))
  (cast `/Game/Weapon/Blueprints/BP_TracerBullet` OtherActor)
  (`SceneComponent.SetVisibility` (`self.PointLight`) false false)
  (`SceneComponent.SetVisibility` (`self.SpotLight`) false false)
  (set `self.Spot1Destroy` true)
  (if (`self.Spot1Destroy`)
    (`KismetSystemLibrary.Delay` 5.0)
    (`SceneComponent.SetVisibility` (`self.PointLight`) true false)
    (`SceneComponent.SetVisibility` (`self.SpotLight`) true false)
    (set `self.Spot1Destroy` false)
    (set `/Game/Blueprints/Player/BP_My_Player.IsDiscover` false (`/Game/Blueprints/Player/FuctionLibrary/BFFL_CallPLayerController.CallMyPlayerCharactere`))
    (set `self.IsTrigger` false)))

(event `self.DeadBoxChase.OnComponentBeginOverlap`
  (params (OverlappedComponent :type "PrimitiveComponent Object Reference") (OtherActor :type "Actor Object Reference") (OtherComp :type "PrimitiveComponent Object Reference") (OtherBodyIndex :type Integer) (bFromSweep :type Boolean) (SweepResult :type "HitResult Structure (by ref)"))
  (bind _asbp_my_player (cast `/Game/Blueprints/Player/BP_My_Player` OtherActor))
  (if (`/Game/Blueprints/Player/BP_My_Player.IsChase` _asbp_my_player)
    (`/Game/Blueprints/Player/BP_My_Player.PlayerDeath` _asbp_my_player)))

(event `Lanceflamme`
  (bind _firesound1 (`self.fireSound1`))
  (if (`self.FireActive`)
    (`/Game/Blueprints/Sounds/BPC_SoundManager.PlaySound` _firesound1 "/Game/Sounds/SonBruts/fire_meca.fire_meca" (`SceneComponent.K2_GetComponentLocation` _firesound1))
    (`SceneComponent.SetVisibility` (`self.Feu1`) true false)
    (`KismetSystemLibrary.Delay` 0.3)
    (`SceneComponent.SetVisibility` (`self.Feu2`) true false)
    (`KismetSystemLibrary.Delay` 0.3)
    (`SceneComponent.SetVisibility` (`self.Feu3`) true false)
    (`KismetSystemLibrary.Delay` 3.0)
    (set `self.FireActive` false)
    (`/Game/Blueprints/Sounds/BPC_SoundManager.StopSound` (`self.fireSound1`))
    (`SceneComponent.SetVisibility` (`self.Feu1`) false false)
    (`SceneComponent.SetVisibility` (`self.Feu2`) false false)
    (`SceneComponent.SetVisibility` (`self.Feu3`) false false)
    (`KismetSystemLibrary.Delay` 6.0)
    (set `self.FireActive` true)))

(fn `Detectiondujoueur`
  (params (self2 :type "SceneComponent Object Reference"))
  (returns (HitActor :type "Actor Object Reference"))
  (bind _returnvalue (`SceneComponent.K2_GetComponentLocation` self2))
  (bind _returnvalue_2 (`SceneComponent.K2_GetComponentLocation` (`Actor.RootComponent` (`GameplayStatics.GetPlayerCharacter` 0))))
  (bind _outhit (`KismetSystemLibrary.LineTraceSingle` :`Start` _returnvalue :`End` (+ _returnvalue_2 (* (`KismetMathLibrary.Normal` (- _returnvalue_2 _returnvalue)) 100.0)) :`TraceChannel` "TraceTypeQuery1" :`bIgnoreSelf` false)) ; Camera Shot
  (return (`.HitActor` (`GameplayStatics.BreakHitResult` _outhit))))

(fn `RotationMechaWhenFocus`
  (bind _pivotbrasdroit (`self.PivotBrasDroit`))
  (bind _pivothaut (`self.PivotHaut`))
  (bind _projecteurdroit (`self.ProjecteurDroit`))
  (bind (_returnvalue_roll _returnvalue_pitch _returnvalue_yaw) (`KismetMathLibrary.BreakRotator` (`KismetMathLibrary.FindLookAtRotation` (`SceneComponent.K2_GetComponentLocation` _pivotbrasdroit) (`SceneComponent.K2_GetComponentLocation` (`Character.CapsuleComponent` (`/Game/Blueprints/Player/FuctionLibrary/BFFL_CallPLayerController.CallMyPlayerCharactere`))))))
  (bind (_returnvalue_roll_2 _returnvalue_pitch_2 _returnvalue_yaw_2) (`KismetMathLibrary.BreakRotator` (`KismetMathLibrary.FindLookAtRotation` (`SceneComponent.K2_GetComponentLocation` _pivothaut) (`SceneComponent.K2_GetComponentLocation` (`Character.CapsuleComponent` (`/Game/Blueprints/Player/FuctionLibrary/BFFL_CallPLayerController.CallMyPlayerCharactere`))))))
  (`SceneComponent.K2_SetWorldRotation` _projecteurdroit (`KismetMathLibrary.FindLookAtRotation` (`SceneComponent.K2_GetComponentLocation` _projecteurdroit) (`SceneComponent.K2_GetComponentLocation` (`Character.CapsuleComponent` (`/Game/Blueprints/Player/FuctionLibrary/BFFL_CallPLayerController.CallMyPlayerCharactere`)))) true true)
  (if (not (`self.Spot1Destroy`))
    (`SceneComponent.K2_SetWorldRotation` _pivothaut (`KismetMathLibrary.MakeRotator` 0.0 0.0 (+ _returnvalue_yaw_2 0.0)) true true)
    (`SceneComponent.K2_SetWorldRotation` _pivotbrasdroit (`KismetMathLibrary.MakeRotator` 0.0 _returnvalue_pitch _returnvalue_yaw) true true)))

(fn `RotationSpot`
  (bind (_relativerotation_roll _relativerotation_pitch _relativerotation_yaw) (`KismetMathLibrary.BreakRotator` (`SceneComponent.RelativeRotation` (`self.ProjecteurDroit`))))
  (bind (_relativerotation_roll_2 _relativerotation_pitch_2 _relativerotation_yaw_2) (`KismetMathLibrary.BreakRotator` (`SceneComponent.RelativeRotation` (`self.ProjecteurDroit`))))
  (if (>= _relativerotation_yaw (`self.RotationMax`))
    (set `self.Addrotation` -0.2)
    (elif (<= _relativerotation_yaw_2 (`self.RotationMin`))
      (set `self.Addrotation` 0.2)))
  (`SceneComponent.K2_AddRelativeRotation` (`self.ProjecteurDroit`) (`KismetMathLibrary.MakeRotator` 0.0 0.0 (`self.Addrotation`)) false false))

(fn `ShootPlayerFocus`
  (bind _returnvalue (`SceneComponent.K2_GetComponentLocation` (`self.Muzzle`)))
  (bind _returnvalue_2 (* (`self.BulletSpreadMecha`) 1.0))
  (bind _returnvalue_3 (* (`self.BulletSpreadMecha`) -1.0))
  (`GameplayStatics.PlaySoundAtLocation` "/Game/Sounds/SCue_Gunmeca.SCue_Gunmeca" (`SceneComponent.K2_GetComponentLocation` (`self.Muzzle`)) (struct) 1.0 1.0 0.0 null null null)
  (bind _output_get (set `self.Vectorshoot` (+ (+ (* (`KismetMathLibrary.Normal` (- (`SceneComponent.K2_GetComponentLocation` (`Actor.RootComponent` (`GameplayStatics.GetPlayerCharacter` 0))) _returnvalue)) 10000.0) _returnvalue) (`KismetMathLibrary.MakeVector` (`KismetMathLibrary.RandomFloatInRange` _returnvalue_3 _returnvalue_2) (`KismetMathLibrary.RandomFloatInRange` _returnvalue_3 _returnvalue_2) (`KismetMathLibrary.RandomFloatInRange` _returnvalue_3 _returnvalue_2)))))
  (bind _outhit (`KismetSystemLibrary.LineTraceSingle` (`SceneComponent.K2_GetComponentLocation` (`self.Muzzle`)) _output_get "TraceTypeQuery1")) ; Shot
  (bind (_bblockinghit _binitialoverlap _time _distance _location _impactpoint _normal _impactnormal _physmat _hitactor) (`GameplayStatics.BreakHitResult` _outhit))
  (bind _asbp_my_player (cast `/Game/Blueprints/Player/BP_My_Player` _hitactor)
    (:`then`
      (`|SpawnActorFromClass` "/Game/Weapon/Blueprints/BP_TracerBullet_Mecha.BP_TracerBullet_Mecha_C" (`KismetMathLibrary.MakeTransform` (`SceneComponent.K2_GetComponentLocation` (`self.Muzzle`)) (`KismetMathLibrary.FindLookAtRotation` (`SceneComponent.K2_GetComponentLocation` (`self.Muzzle`)) (`SceneComponent.K2_GetComponentLocation` (`Character.CapsuleComponent` (`/Game/Blueprints/Player/FuctionLibrary/BFFL_CallPLayerController.CallMyPlayerCharactere`)))) (0.25 0.25 0.25)) "Undefined" "OverrideRootScale" null null)
      (`KismetSystemLibrary.PrintString` "Hello")
      (`/Game/Blueprints/Player/BP_My_Player.PlayerDeath` _asbp_my_player))
    (:`CastFailed`
      (`|SpawnActorFromClass` "/Game/Weapon/Blueprints/BP_DecalBullet.BP_DecalBullet_C" (`KismetMathLibrary.MakeTransform` _impactpoint (`KismetMathLibrary.Conv_VectorToRotator` _impactpoint) (0.025 0.025 0.025)) "Undefined" "OverrideRootScale" null null)
      (`|SpawnActorFromClass` "/Game/Weapon/Blueprints/BP_TracerBullet_Mecha.BP_TracerBullet_Mecha_C" (`KismetMathLibrary.MakeTransform` (`SceneComponent.K2_GetComponentLocation` (`self.Muzzle`)) (`KismetMathLibrary.FindLookAtRotation` (`SceneComponent.K2_GetComponentLocation` (`self.Muzzle`)) _impactpoint) (0.5 0.5 0.5)) "Undefined" "OverrideRootScale" null null))))

(fn `UserConstructionScript`)