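; Mech enemy with a searchlight that sweeps between yaw limits to detect the player.
; Cone overlap with a line-of-sight trace flags the player discovered; while alerted, light, upper body and right arm track them in the detection color.
; Losing sight clears detection after a delay.
; Tracer bullets hitting its sphere hide the light and halt body tracking for five seconds, then clear the alert; blackboard setup is unconnected.
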(event `self.ReceiveBeginPlay`
  (set `self.DefautRotProjDroite` (`SceneComponent.K2_GetComponentRotation` (`self.ProjecteurDroit`)))
  (set `self.DefautRotMeca` (`SceneComponent.K2_GetComponentRotation` (`self.PivotHaut`)))
  (set `self.DefautRotBrasDroite` (`SceneComponent.K2_GetComponentRotation` (`self.PivotBrasDroit`))))

(event `self.ReceiveTick`
  (params (DeltaSeconds :type "Float (single-precision)"))
  (bind _myplayercharactere (`/Game/Blueprints/Player/FuctionLibrary/BFFL_CallPLayerController.CallMyPlayerCharactere`))
  (bind _myplayercharactere_2 (`/Game/Blueprints/Player/FuctionLibrary/BFFL_CallPLayerController.CallMyPlayerCharactere`))
  (bind _pivotbrasdroit (`self.PivotBrasDroit`))
  (bind _pivothaut (`self.PivotHaut`))
  (bind _spotlight (`self.SpotLight`))
  (bind (_relativerotation_roll _relativerotation_pitch _relativerotation_yaw) (`KismetMathLibrary.BreakRotator` (`SceneComponent.RelativeRotation` (`self.ProjecteurDroit`))))
  (bind (_relativerotation_roll_2 _relativerotation_pitch_2 _relativerotation_yaw_2) (`KismetMathLibrary.BreakRotator` (`SceneComponent.RelativeRotation` (`self.ProjecteurDroit`))))
  (bind (_returnvalue_roll _returnvalue_pitch _returnvalue_yaw) (`KismetMathLibrary.BreakRotator` (`KismetMathLibrary.FindLookAtRotation` (`SceneComponent.K2_GetComponentLocation` _pivothaut) (`SceneComponent.K2_GetComponentLocation` (`Character.CapsuleComponent` (`/Game/Blueprints/Player/FuctionLibrary/BFFL_CallPLayerController.CallMyPlayerCharactere`))))))
  (bind (_returnvalue_roll_2 _returnvalue_pitch_2 _returnvalue_yaw_2) (`KismetMathLibrary.BreakRotator` (`KismetMathLibrary.FindLookAtRotation` (`SceneComponent.K2_GetComponentLocation` _pivotbrasdroit) (`SceneComponent.K2_GetComponentLocation` (`Character.CapsuleComponent` (`/Game/Blueprints/Player/FuctionLibrary/BFFL_CallPLayerController.CallMyPlayerCharactere`))))))
  (if (and (not (`/Game/Blueprints/Player/BP_My_Player.IsChase` _myplayercharactere_2)) (not (`/Game/Blueprints/Player/BP_My_Player.IsDiscover` _myplayercharactere_2)) (not (`self.IsTrigger`)))
    (if (>= _relativerotation_yaw_2 (`self.RotationMax`))
      (set `self.Addrotation` -0.2)
      (elif (<= _relativerotation_yaw (`self.RotationMin`))
        (set `self.Addrotation` 0.2)))
    (`SceneComponent.K2_AddRelativeRotation` (`self.ProjecteurDroit`) (`KismetMathLibrary.MakeRotator` 0.0 0.0 (`self.Addrotation`)) false false)
    (if (not (`self.ResetCourse`))
      (`LightComponent.SetLightColor` (`self.PointLight`) (`self.DefaultColor`) true)
      (`LightComponent.SetLightColor` (`self.SpotLight`) (`self.DefaultColor`) true)
      (`SceneComponent.K2_SetWorldRotation` (`self.SpotLight`) (`self.DefautRotProjDroite`) false false)
      (`SceneComponent.K2_SetWorldRotation` (`self.PointLight`) (`self.DefautRotProjDroite`) false false)
      (`SceneComponent.K2_SetWorldRotation` (`self.PivotBrasDroit`) (`self.DefautRotBrasDroite`) false false)
      (`SceneComponent.K2_SetWorldRotation` (`self.PivotHaut`) (`self.DefautRotMeca`) false false)
      (set `self.ResetCourse` true))
    (else
      (set `self.ResetCourse` false)
      (`|ExecutionSequence`
        (:`then_0`
          (`SceneComponent.K2_SetWorldRotation` _spotlight (`KismetMathLibrary.FindLookAtRotation` (`SceneComponent.K2_GetComponentLocation` _spotlight) (`SceneComponent.K2_GetComponentLocation` (`Character.CapsuleComponent` (`/Game/Blueprints/Player/FuctionLibrary/BFFL_CallPLayerController.CallMyPlayerCharactere`)))) true true)
          (if (not (`self.Spot1Destroy`))
            (`SceneComponent.K2_SetWorldRotation` _pivothaut (`KismetMathLibrary.MakeRotator` 0.0 0.0 (+ _returnvalue_yaw 0.0)) true true)
            (`SceneComponent.K2_SetWorldRotation` _pivotbrasdroit (`KismetMathLibrary.MakeRotator` 0.0 _returnvalue_pitch_2 _returnvalue_yaw_2) true true)))
        (:`then_1`
          (`LightComponent.SetLightColor` (`self.SpotLight`) (`self.DetectColor`) true)
          (`LightComponent.SetLightColor` (`self.PointLight`) (`self.DetectColor`) true))
        (:`then_2`
          (bind _hitactor (`self.Detectiondujoueur` (`self.SpotLight`)))
          (cast `/Game/Blueprints/Player/BP_My_Player` _hitactor
            (:`then`
              (set `self.Joueurcacher` false))
            (:`CastFailed`
              (set `self.Joueurcacher` true)))
          (if (not (`self.Joueurcacher`))
            (set `/Game/Blueprints/Player/BP_My_Player.IsDiscover` true _myplayercharactere)
            (set `self.IsTrigger` true)
            (else
              (`KismetSystemLibrary.Delay` 5.0)
              (set `/Game/Blueprints/Player/BP_My_Player.IsDiscover` false _myplayercharactere)
              (set `self.IsTrigger` false))))))))

(event `self.ConeDroite.OnComponentBeginOverlap`
  (params (OverlappedComponent :type "PrimitiveComponent Object Reference") (OtherActor :type "Actor Object Reference") (OtherComp :type "PrimitiveComponent Object Reference") (OtherBodyIndex :type Integer) (bFromSweep :type Boolean) (SweepResult :type "HitResult Structure (by ref)"))
  (cast `/Game/Blueprints/Player/BP_My_Player` OtherActor)
  (if (not (`self.Joueurcacher`))
    (bind _hitactor (`self.Detectiondujoueur` (`self.SpotLight`)))
    (cast `/Game/Blueprints/Player/BP_My_Player` _hitactor)
    (set `self.IsTrigger` true)
    (set `/Game/Blueprints/Player/BP_My_Player.IsDiscover` true (`/Game/Blueprints/Player/FuctionLibrary/BFFL_CallPLayerController.CallMyPlayerCharactere`))))

(event `self.Sphere.OnComponentBeginOverlap`
  (params (OverlappedComponent :type "PrimitiveComponent Object Reference") (OtherActor :type "Actor Object Reference") (OtherComp :type "PrimitiveComponent Object Reference") (OtherBodyIndex :type Integer) (bFromSweep :type Boolean) (SweepResult :type "HitResult Structure (by ref)"))
  (cast `/Game/Weapon/Blueprints/BP_TracerBullet` OtherActor)
  (`SceneComponent.SetVisibility` (`self.PointLight`) false false)
  (`SceneComponent.SetVisibility` (`self.SpotLight`) false false)
  (set `self.Spot1Destroy` true)
  (if (`self.Spot1Destroy`)
    (`KismetSystemLibrary.Delay` 5.0)
    (`SceneComponent.SetVisibility` (`self.PointLight`) true false)
    (`SceneComponent.SetVisibility` (`self.SpotLight`) true false)
    (set `self.Spot1Destroy` false)
    (set `/Game/Blueprints/Player/BP_My_Player.IsDiscover` false (`/Game/Blueprints/Player/FuctionLibrary/BFFL_CallPLayerController.CallMyPlayerCharactere`))
    (set `self.IsTrigger` false)))

(fn `Detectiondujoueur`
  (params (self2 :type "SceneComponent Object Reference"))
  (returns (HitActor :type "Actor Object Reference"))
  (bind _returnvalue (`SceneComponent.K2_GetComponentLocation` self2))
  (bind _returnvalue_2 (`SceneComponent.K2_GetComponentLocation` (`Actor.RootComponent` (`GameplayStatics.GetPlayerCharacter` 0))))
  (bind _outhit (`KismetSystemLibrary.LineTraceSingle` :`Start` _returnvalue :`End` (+ _returnvalue_2 (* (`KismetMathLibrary.Normal` (- _returnvalue_2 _returnvalue)) 100.0)) :`TraceChannel` "TraceTypeQuery1" :`bIgnoreSelf` false)) ; Camera Shot
  (return (`.HitActor` (`GameplayStatics.BreakHitResult` _outhit))))

(fn `UserConstructionScript`)