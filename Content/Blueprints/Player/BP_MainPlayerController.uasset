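; Main player controller that routes player input and handles respawning at checkpoints.
; Caches the BP_My_Player character on BeginPlay and relays movement, look, weapon, gas mask and pause inputs through dedicated Call events.
; ReloadFromCheckPoint looks up the last checkpoint in the CheckPointManager map.
; If found, it unpauses, hides the cursor, clears the player's death flag and moves them to that checkpoint's transform.
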(event `self.ReceiveBeginPlay`
  (bind _asbp_my_player (cast `/Game/Blueprints/Player/BP_My_Player` (`GameplayStatics.GetPlayerCharacter` 0)))
  (set `self.PlayerCarachere` _asbp_my_player))

(event `InputAxis|Mouse - Look Up/Down`
  (params (AxisValue :type "Float (single-precision)"))
  ;[1 1 1] Mouse - Input
  (`self.AxisMouseUpDown` AxisValue))

(event `InputAxis|Keyboard - Forward/Backward`
  (params (AxisValue :type "Float (single-precision)"))
  ;[1 1 1] Keeyboard - Input
  (`self.KeyBoardForwardBackward` AxisValue))

(event `InputAxis|Keyboard - Right/Left`
  (params (AxisValue :type "Float (single-precision)"))
  ;[1 1 1] Keeyboard - Input
  (`self.KeyBoardRightLeft` AxisValue))

(event `InputAxis|Mouse - Look Right/Left`
  (params (AxisValue :type "Float (single-precision)"))
  ;[1 1 1] Mouse - Input
  (`self.AxisMouseRightLeft` AxisValue))

(event `InputAction|EquipWeapon`
  (params (Key :type "Key Structure"))
  ;[1 1 1] Weapon - Input
  (:`Pressed`
    (`self.EquipeArme`)))

(event `InputAction|Masque a Gaz`
  (params (Key :type "Key Structure"))
  ;[1 1 1] Equipe Maque a Gaz - Input
  (:`Pressed`
    (`self.MasqueGaz`)))

(event `InputAction|Fire`
  (params (Key :type "Key Structure"))
  ;[1 1 1] Weapon - Input
  (:`Pressed`
    (`self.Tir`)))

(event `InputAction|Reload`
  (params (Key :type "Key Structure"))
  ;[1 1 1] Weapon - Input
  (:`Pressed`
    (`self.Recharge`)))

(event `InputAction|PauseMenu`
  (params (Key :type "Key Structure"))
  (:`Pressed`
    (`self.MenuPause`)))

(fn `ReloadFromCheckPoint`
  (bind _myplayercharactere (`/Game/Blueprints/Player/FuctionLibrary/BFFL_CallPLayerController.CallMyPlayerCharactere`))
  (bind (_value _returnvalue) (`BlueprintMapLibrary.Map_Find` (`/Game/Blueprints/RespawnPlayer/BP_CheckPointManager.CheckPointMap` (`self.CheckPointManager`)) (`self.LastCheckPoint`)))
  (if _returnvalue
    (`GameplayStatics.SetGamePaused` false)
    (set `PlayerController.bShowMouseCursor` false (`GameplayStatics.GetPlayerController` 0))
    (set `/Game/Blueprints/Player/BP_My_Player.IsDead` false _myplayercharactere)
    (`self.K2_SetActorTransform` _myplayercharactere (`self.GetTransform` _value) false false)))

(fn `UserConstructionScript`)