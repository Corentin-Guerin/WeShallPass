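; First-person player character with walking, sprinting, jumping, three stances, interaction, a pistol and a filter-consuming gas mask.
; Movement, look and weapon inputs bind to main player controller dispatchers on BeginPlay, where the weapon also spawns hidden in the hand.
; Tick interpolates capsule, speed and camera height per stance, with upward traces blocking rising under obstacles.
; A per-tick camera trace selects the interactable component, toggling its feedback.
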(event `self.ReceiveBeginPlay`
  (`self.DefaultMouseBinding`)
  (`self.DefaultKeyboardRighLeftBinding`)
  (`self.DefaultKeyboardForwardBackwardBinding`)
  (`self.DefaultGKey`)
  (`self.DefaultLeftclic`)
  (`self.DefaultAKey`)
  (`self.DefaultRKey`)
  (`self.SpawnWeapon`))

(event `self.ReceiveTick`
  (params (DeltaSeconds :type "Float (single-precision)"))
  (`self.Crouch Crawl Runtime`)
  (`self.CrouchTrace`)
  (`self.CrawlTrace`)
  (`self.TickForInteraction` DeltaSeconds))

(event `DefaultEchapKey`
  (clear `/Game/Blueprints/Player/BP_MainPlayerController.MenuPause` (`/Game/Blueprints/Player/FuctionLibrary/BFFL_CallPLayerController.CallMainPlayerController`)))

(event `KeyboardUpDownMove`
  (params (Value :type "Float (double-precision)"))
  (bind _returnvalue (`GameplayStatics.GetPlayerController` 0))
  ;[1 1 1] Keeyboard - Input
  (`self.AddMovementInput` (`KismetMathLibrary.GetForwardVector` (`KismetMathLibrary.MakeRotator` 0.0 0.0 (.yaw (`self.GetControlRotation`)))) Value)
  (`PlayerController.ClientStartCameraShake` :`self` _returnvalue :`Shake` "/Game/Blueprints/Camera/BP_MyCameraShake_01valide.BP_MyCameraShake_01valide_C" :`Scale` Value)
  (`PlayerController.ClientStartCameraShake` :`self` _returnvalue :`Shake` "/Game/Blueprints/Camera/BP_MyCameraShake_01valide.BP_MyCameraShake_01valide_C" :`Scale` (* Value -1.0)))

(event `KeyboardRightLeftMove`
  (params (Value :type "Float (double-precision)"))
  (bind _returnvalue (`GameplayStatics.GetPlayerController` 0))
  ;[1 1 1] Keeyboard - Input
  (`self.AddMovementInput` (`KismetMathLibrary.GetRightVector` (`KismetMathLibrary.MakeRotator` 0.0 0.0 (.yaw (`self.GetControlRotation`)))) Value)
  (`PlayerController.ClientStartCameraShake` :`self` _returnvalue :`Shake` "/Game/Blueprints/Camera/BP_MyCameraShake_01valide.BP_MyCameraShake_01valide_C" :`Scale` Value)
  (`PlayerController.ClientStartCameraShake` :`self` _returnvalue :`Shake` "/Game/Blueprints/Camera/BP_MyCameraShake_01valide.BP_MyCameraShake_01valide_C" :`Scale` (* Value -1.0)))

(event `MouseLookUPDown`
  (params (Val :type "Float (double-precision)"))
  ;[1 1 1] Rotation Camera playeur
  (`self.AddControllerPitchInput` Val))

(event `InputAction|Sprint`
  (params (Key :type "Key Structure"))
  ;[1 1 1] S'accroupire / Sprint / Jump
  (:`Pressed`
    (`self.Sprint` :!label _label))
  (:`Released`
    (goto _label :!via `Released`)))

(event `InputAction|Crouch`
  (params (Key :type "Key Structure"))
  ;[1 1 1] S'accroupire / Sprint / Jump
  (:`Pressed`
    (`self.Crouchs`)))

(event `MouseLookRightLeft`
  (params (Val :type "Float (double-precision)"))
  ;[1 1 1] Rotation Camera playeur
  (`self.AddControllerYawInput` Val))

(event `InputAction|Jump`
  (params (Key :type "Key Structure"))
  ;[1 1 1] S'accroupire / Sprint / Jump
  (:`Pressed`
    (`self.Jumps` :!label _label_2))
  (:`Released`
    (goto _label_2 :!via `Released`)))

(event `DefaultMouseBinding`
  (bind _mainplayercontroller (`/Game/Blueprints/Player/FuctionLibrary/BFFL_CallPLayerController.CallMainPlayerController`))
  ;[1 1 1] Default Mouse binding - Axis Mouse
  (clear `/Game/Blueprints/Player/BP_MainPlayerController.AxisMouseRightLeft` _mainplayercontroller)
  (clear `/Game/Blueprints/Player/BP_MainPlayerController.AxisMouseUpDown` _mainplayercontroller)
  (add `/Game/Blueprints/Player/BP_MainPlayerController.AxisMouseRightLeft` _mainplayercontroller (`|CreateDelegate` :!event `MouseLookRightLeft`))
  (add `/Game/Blueprints/Player/BP_MainPlayerController.AxisMouseUpDown` _mainplayercontroller (`|CreateDelegate` :!event `MouseLookUPDown`)))

(event `DefaultKeyboardForwardBackwardBinding`
  (bind _mainplayercontroller (`/Game/Blueprints/Player/FuctionLibrary/BFFL_CallPLayerController.CallMainPlayerController`))
  ;[1 1 1] Default Mouse binding - Axis Mouse
  (clear `/Game/Blueprints/Player/BP_MainPlayerController.KeyBoardForwardBackward` _mainplayercontroller)
  (add `/Game/Blueprints/Player/BP_MainPlayerController.KeyBoardForwardBackward` _mainplayercontroller (`|CreateDelegate` :!event `KeyboardUpDownMove`)))

(event `DefaultKeyboardRighLeftBinding`
  (bind _mainplayercontroller (`/Game/Blueprints/Player/FuctionLibrary/BFFL_CallPLayerController.CallMainPlayerController`))
  ;[1 1 1] Default Mouse binding - Axis Mouse
  (clear `/Game/Blueprints/Player/BP_MainPlayerController.KeyBoardRightLeft` _mainplayercontroller)
  (add `/Game/Blueprints/Player/BP_MainPlayerController.KeyBoardRightLeft` _mainplayercontroller (`|CreateDelegate` :!event `KeyboardRightLeftMove`)))

(event `EquipeMasqueAGaz`
  (bind _filteramount (`self.FilterAmount`))
  ;[1 1 1] Equpie Maque a Gaz
  (`/Engine/EditorBlueprintResources/StandardMacros.FlipFlop`
    (:`A`
      (if (>= _filteramount 1)
        (set `self.IsMasked` true)
        (set `self.FilterAmount` (- _filteramount 1))
        ;;[1 1 1] ajouter animation du masque
        (`KismetMaterialLibrary.SetScalarParameterValue` "/Game/Textures/Material/MPC_Gaz.MPC_Gaz" "Opacity" 1.0)
        (set `self.AnimEnCours` false)
        (if (`self.IsInGaz`)
          (set `self.EquipMaskInGaz` true))))
    (:`B`
      (set `self.IsMasked` false)
      (`KismetMaterialLibrary.SetScalarParameterValue` "/Game/Textures/Material/MPC_Gaz.MPC_Gaz" "Opacity")
      (set `self.AnimEnCours` false)
      (if (`self.IsInGaz`)
        (set `self.EquipMaskInGaz` false)))))

(event `DefaultGKey`
  ;[1 1 1] Default Touche [G] - Equipe Masque a Gaz
  (clear `/Game/Blueprints/Player/BP_MainPlayerController.MasqueGaz` (`/Game/Blueprints/Player/FuctionLibrary/BFFL_CallPLayerController.CallMainPlayerController`)))

(event `InputAction|Interact`
  (params (Key :type "Key Structure"))
  (:`Pressed`
    (`/Engine/EditorBlueprintResources/StandardMacros.IsValid` (`self.CurentInteractable`)
      (:`Is Valid`
        (`/Game/Blueprints/Intercatible/BP_C_Interactable.Interact` (`self.CurentInteractable`) self)))))

(event `TickForInteraction`
  (params (`Delta Seconds` :type "Float (double-precision)"))
  (bind _camera (`self.Camera`))
  (bind _returnvalue (`SceneComponent.K2_GetComponentLocation` _camera))
  (bind (_outhit _returnvalue_2) (`KismetSystemLibrary.LineTraceSingle` _returnvalue (+ _returnvalue (* (`SceneComponent.GetForwardVector` _camera) (`self.InterctDirectionLenght`))) "TraceTypeQuery1"))
  (if _returnvalue_2
    (bind _asbp_c_interactable (cast `/Game/Blueprints/Intercatible/BP_C_Interactable` (`.HitComponent` (`GameplayStatics.BreakHitResult` _outhit)))
      (:`then`
        (if (not (== _asbp_c_interactable (`self.CurentInteractable`)))
          (`self.UnFeedBackInterractable`)
          (bind _output_get (set `self.CurentInteractable` _asbp_c_interactable))
          (`/Game/Blueprints/Intercatible/BP_C_Interactable.CanInteractFeedBack` _output_get)))
      (:`CastFailed`
        (`self.UnFeedBackInterractable` :!label _label)))
    (else
      (goto _label))))

(event `UnFeedBackInterractable`
  (bind _curentinteractable (`self.CurentInteractable`))
  (`/Engine/EditorBlueprintResources/StandardMacros.IsValid` _curentinteractable
    (:`Is Valid`
      (`/Game/Blueprints/Intercatible/BP_C_Interactable.CantInteractFeedBack` _curentinteractable)
      (set `self.CurentInteractable` null))))

(event `EquipWeapon`
  (bind _primaryweapon (`self.PrimaryWeapon`))
  ;[1 1 1] Equipe/Unequipe Weapon
  (if (`self.CanEquipWeapon`)
    (`/Engine/EditorBlueprintResources/StandardMacros.FlipFlop`
      (:`A`
        (set `self.HaveWeapon` true)
        (`SceneComponent.SetVisibility` (`Actor.RootComponent` _primaryweapon) true false)
        (bind _returnvalue (`|CreateWidget` "/Game/UI/InGame/HUD_MuniWeapon.HUD_MuniWeapon_C"))
        (`UserWidget.AddToViewport` _returnvalue 0))
      (:`B`
        (set `self.HaveWeapon` false)
        (`SceneComponent.SetVisibility` (`Actor.RootComponent` _primaryweapon) false false)
        (`Widget.RemoveFromParent` _returnvalue)))))

(event `Fire`
  (bind _primaryweapon (`self.PrimaryWeapon`))
  ;[1 1 1] Tir
  (if (and (`self.HaveWeapon`) (not (`self.IsReloading`)))
    (set `self.IsShooting` true)
    (`/Game/Weapon/Blueprints/BP_WeaponBase.Fire` _primaryweapon)
    (if (> (`/Game/Weapon/Blueprints/BP_WeaponBase.Ammocount` _primaryweapon) 0)
      (`|PlayMontage` (`self.SkeletalMesh`) "/Game/Animation/Arms/ArmsWeapon/Arms_Glock_Fire_anim_Montage.Arms_Glock_Fire_anim_Montage"
        (:`then`
          (set `self.IsShooting` false))))))

(event `Reload`
  (bind _primaryweapon (`self.PrimaryWeapon`))
  (bind _primaryweapon_2 (`self.PrimaryWeapon`))
  ;[1 1 1] Recharge
  (if (`self.HaveWeapon`)
    (if (and (< (`/Game/Weapon/Blueprints/BP_WeaponBase.Ammocount` _primaryweapon) (`/Game/Weapon/Blueprints/BP_WeaponBase.AmmoChargeur` _primaryweapon)) (> (`/Game/Weapon/Blueprints/BP_WeaponBase.MaxAmmo` _primaryweapon) 0))
      (`/Engine/EditorBlueprintResources/StandardMacros.DoOnce` false :!label _label
        (:`Completed`
          (set `self.IsReloading` true)
          (`AnimInstance.Montage_Play` (`SkeletalMeshComponent.GetAnimInstance` (`self.SkeletalMesh`)) "/Game/Animation/Arms/ArmsWeapon/Arms_Glock_Reload_anim_Montage.Arms_Glock_Reload_anim_Montage" 1.0 "MontageLength" 0.0 true)
          (`/Game/Weapon/Blueprints/BP_WeaponBase.Reload` _primaryweapon_2)
          (`KismetSystemLibrary.Delay` (`/Game/Weapon/Blueprints/BP_WeaponBase.ReloadTime` _primaryweapon_2))
          (set `self.IsReloading` false)
          (goto _label :!via `Reset`))))))

(event `DefaultAKey`
  (bind _mainplayercontroller (`/Game/Blueprints/Player/FuctionLibrary/BFFL_CallPLayerController.CallMainPlayerController`))
  (clear `/Game/Blueprints/Player/BP_MainPlayerController.EquipeArme` _mainplayercontroller)
  (add `/Game/Blueprints/Player/BP_MainPlayerController.EquipeArme` _mainplayercontroller (`|CreateDelegate` :!event `EquipWeapon`)))

(event `DefaultLeftclic`
  (bind _mainplayercontroller (`/Game/Blueprints/Player/FuctionLibrary/BFFL_CallPLayerController.CallMainPlayerController`))
  (clear `/Game/Blueprints/Player/BP_MainPlayerController.Tir` _mainplayercontroller)
  (add `/Game/Blueprints/Player/BP_MainPlayerController.Tir` _mainplayercontroller (`|CreateDelegate` :!event `Fire`)))

(event `DefaultRKey`
  (bind _mainplayercontroller (`/Game/Blueprints/Player/FuctionLibrary/BFFL_CallPLayerController.CallMainPlayerController`))
  (clear `/Game/Blueprints/Player/BP_MainPlayerController.Recharge` _mainplayercontroller)
  (add `/Game/Blueprints/Player/BP_MainPlayerController.Recharge` _mainplayercontroller (`|CreateDelegate` :!event `Reload`)))

(fn `CrawlTrace`
  (bind _returnvalue (- (`self.K2_GetActorLocation`) (0.0 20.0 0.0)))
  (bind _returnvalue_2 (- (`self.K2_GetActorLocation`) (20.0 0.0 0.0)))
  (bind _returnvalue_3 (+ (`self.K2_GetActorLocation`) (20.0 0.0 0.0)))
  (bind _returnvalue_4 (+ (`self.K2_GetActorLocation`) (0.0 20.0 0.0)))
  (bind (_outhit _returnvalue_5) (`KismetSystemLibrary.LineTraceSingle` _returnvalue_3 (+ _returnvalue_3 (* (`self.GetActorUpVector`) 34.0)) "TraceTypeQuery1"))
  (set `self.CrawlBlock01` _returnvalue_5)
  (bind (_outhit_2 _returnvalue_6) (`KismetSystemLibrary.LineTraceSingle` _returnvalue_2 (+ _returnvalue_2 (* (`self.GetActorUpVector`) 34.0)) "TraceTypeQuery1"))
  (set `self.CrawlBlock02` _returnvalue_6)
  (bind (_outhit_3 _returnvalue_7) (`KismetSystemLibrary.LineTraceSingle` _returnvalue_4 (+ _returnvalue_4 (* (`self.GetActorUpVector`) 34.0)) "TraceTypeQuery1"))
  (set `self.CrawlBlock03` _returnvalue_7)
  (bind (_outhit_4 _returnvalue_8) (`KismetSystemLibrary.LineTraceSingle` _returnvalue (+ _returnvalue (* (`self.GetActorUpVector`) 34.0)) "TraceTypeQuery1"))
  (set `self.CrawlBlock04` _returnvalue_8))

(fn `Crouch Crawl Runtime`
  (bind _camera (`self.Camera`))
  (bind (_relativelocation_x _relativelocation_y _relativelocation_z) (`KismetMathLibrary.BreakVector` (`SceneComponent.RelativeLocation` _camera)))
  (`CapsuleComponent.SetCapsuleSize` (`self.CapsuleComponent`) (`KismetMathLibrary.FInterpTo_Constant` (`CapsuleComponent.CapsuleRadius` (`self.CapsuleComponent`)) (select `/Game/Data/Enume_Mouvement` (`self.CrouchStates`) :`NewEnumerator0` (`self.StandRadius`) :`NewEnumerator1` (`self.CrouchRadius`) :`NewEnumerator2` (`self.CrawlRadius`)) (`GameplayStatics.GetWorldDeltaSeconds`) (`self.InterpSpeed`)) (`KismetMathLibrary.FInterpTo_Constant` (`CapsuleComponent.CapsuleHalfHeight` (`self.CapsuleComponent`)) (select `/Game/Data/Enume_Mouvement` (`self.CrouchStates`) :`NewEnumerator0` (`self.StandHalfHeight`) :`NewEnumerator1` (`self.CrouchHalfHeight`) :`NewEnumerator2` (`self.CrawlHalfHeight`)) (`GameplayStatics.GetWorldDeltaSeconds`) (`self.InterpSpeed`)) true)
  (set `CharacterMovementComponent.MaxWalkSpeed` (`KismetMathLibrary.FInterpTo_Constant` (`CharacterMovementComponent.MaxWalkSpeed` (`self.CharacterMovement`)) (select `/Game/Data/Enume_Mouvement` (`self.CrouchStates`) :`NewEnumerator0` (select `bool` (`self.IsSprinting`) :`false` (`self.WalkSpeed`) :`true` (`self.SprintSpeed`)) :`NewEnumerator1` (`self.CrouchSpeed`) :`NewEnumerator2` (`self.CrawlSpeed`)) (`GameplayStatics.GetWorldDeltaSeconds`) (* (`self.InterpSpeed`) 5.0)) (`self.CharacterMovement`))
  (`SceneComponent.K2_SetRelativeLocation` _camera (`KismetMathLibrary.MakeVector` _relativelocation_x _relativelocation_y (`KismetMathLibrary.FInterpTo_Constant` _relativelocation_z (select `/Game/Data/Enume_Mouvement` (`self.CrouchStates`) :`NewEnumerator0` (`self.CameraLocationStand`) :`NewEnumerator1` (`self.CameraLocationCrouch`) :`NewEnumerator2` (`self.CameraLocationCrawl`)) (`GameplayStatics.GetWorldDeltaSeconds`) (`self.InterpSpeed`))) false false))

(fn `CrouchTrace`
  (bind _crouchhalfheight (`self.CrouchHalfHeight`))
  (bind _crouchhalfheight_2 (`self.CrouchHalfHeight`))
  (bind _crouchhalfheight_3 (`self.CrouchHalfHeight`))
  (bind _crouchhalfheight_4 (`self.CrouchHalfHeight`))
  (bind _returnvalue (- (`self.K2_GetActorLocation`) (0.0 34.0 0.0)))
  (bind _returnvalue_2 (- (`self.K2_GetActorLocation`) (34.0 0.0 0.0)))
  (bind _returnvalue_3 (+ (`self.K2_GetActorLocation`) (34.0 0.0 0.0)))
  (bind _returnvalue_4 (* _crouchhalfheight_3 2.3))
  (bind _returnvalue_5 (* _crouchhalfheight_4 2.3))
  (bind _returnvalue_6 (* _crouchhalfheight 2.3))
  (bind _returnvalue_7 (+ (`self.K2_GetActorLocation`) (0.0 34.0 0.0)))
  (bind _returnvalue_8 (* _crouchhalfheight_2 2.3))
  (bind (_outhit _returnvalue_9) (`KismetSystemLibrary.LineTraceSingle` _returnvalue_3 (+ _returnvalue_3 (* (`self.GetActorUpVector`) (select `/Game/Data/Enume_Mouvement` (`self.CrouchStates`) :`NewEnumerator0` _returnvalue_4 :`NewEnumerator1` _returnvalue_4 :`NewEnumerator2` (* _crouchhalfheight_3 2.8)))) "TraceTypeQuery1"))
  (set `self.CrouchBlock01` _returnvalue_9)
  (bind (_outhit_2 _returnvalue_10) (`KismetSystemLibrary.LineTraceSingle` _returnvalue_2 (+ _returnvalue_2 (* (`self.GetActorUpVector`) (select `/Game/Data/Enume_Mouvement` (`self.CrouchStates`) :`NewEnumerator0` _returnvalue_5 :`NewEnumerator1` _returnvalue_5 :`NewEnumerator2` (* _crouchhalfheight_4 2.8)))) "TraceTypeQuery1"))
  (set `self.CrouchBlock02` _returnvalue_10)
  (bind (_outhit_3 _returnvalue_11) (`KismetSystemLibrary.LineTraceSingle` _returnvalue_7 (+ _returnvalue_7 (* (`self.GetActorUpVector`) (select `/Game/Data/Enume_Mouvement` (`self.CrouchStates`) :`NewEnumerator0` _returnvalue_8 :`NewEnumerator1` _returnvalue_8 :`NewEnumerator2` (* _crouchhalfheight_2 2.8)))) "TraceTypeQuery1"))
  (set `self.CrouchBlock03` _returnvalue_11)
  (bind (_outhit_4 _returnvalue_12) (`KismetSystemLibrary.LineTraceSingle` _returnvalue (+ _returnvalue (* (`self.GetActorUpVector`) (select `/Game/Data/Enume_Mouvement` (`self.CrouchStates`) :`NewEnumerator0` _returnvalue_6 :`NewEnumerator1` _returnvalue_6 :`NewEnumerator2` (* _crouchhalfheight 2.8)))) "TraceTypeQuery1"))
  (set `self.CrouchBlock04` _returnvalue_12))

(fn `SpawnWeapon`
  (bind _returnvalue (`|SpawnActorFromClass` "/Game/Weapon/Blueprints/BP_Weapon.BP_Weapon_C" (`KismetMathLibrary.MakeTransform` (0.0 0.0 0.0)) "Undefined" "OverrideRootScale" null null))
  (bind _output_get (set `self.PrimaryWeapon` _returnvalue))
  (`self.K2_AttachToComponent` _output_get (`self.SkeletalMesh`) "Palm_R" "KeepRelative" "KeepRelative" "KeepRelative" true)
  (`SceneComponent.SetVisibility` (`Actor.RootComponent` (`self.PrimaryWeapon`)) false false))

(fn `Toggle Crouch`
  (params (IsLieDonw :type Boolean))
  (if IsLieDonw
    (`self.Crouch`)
    (else
      (`self.UnCrouch`))))

(fn `UserConstructionScript`)