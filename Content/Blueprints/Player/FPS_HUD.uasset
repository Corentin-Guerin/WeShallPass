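; FPS HUD that adds the crosshair widget to the viewport on BeginPlay and handles the pause menu.
; It rebinds to the MenuPause dispatcher on the main player controller, clearing existing bindings first.
; The Pausemenu event uses a FlipFlop to alternately create or remove the pause widget, toggling game pause and mouse cursor visibility with it.
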(event `self.ReceiveBeginPlay`
  (`self.BindEchapKey`)
  (bind _returnvalue (`|CreateWidget` "/Game/UI/InGame/WBP_CrossHair.WBP_CrossHair_C"))
  (`UserWidget.AddToViewport` _returnvalue 0))

(event `Pausemenu`
  (bind _returnvalue (`GameplayStatics.GetPlayerController` 0))
  ;[1 1 1] Pause Menu
  (`/Engine/EditorBlueprintResources/StandardMacros.FlipFlop`
    (:`A`
      (bind _returnvalue_2 (`|CreateWidget` "/Game/UI/InGame/WBP_Pause_Menu_Widget.WBP_Pause_Menu_Widget_C"))
      (`UserWidget.AddToViewport` _returnvalue_2 0)
      (`GameplayStatics.SetGamePaused` true)
      (set `PlayerController.bShowMouseCursor` true _returnvalue))
    (:`B`
      (`Widget.RemoveFromParent` _returnvalue_2)
      (`GameplayStatics.SetGamePaused` false)
      (set `PlayerController.bShowMouseCursor` false _returnvalue))))

(event `BindEchapKey`
  (bind _mainplayercontroller (`/Game/Blueprints/Player/FuctionLibrary/BFFL_CallPLayerController.CallMainPlayerController`))
  ;[1 1 1] Pause Menu
  (clear `/Game/Blueprints/Player/BP_MainPlayerController.MenuPause` _mainplayercontroller)
  (add `/Game/Blueprints/Player/BP_MainPlayerController.MenuPause` _mainplayercontroller (`|CreateDelegate` :!event `Pausemenu`)))

(fn `UserConstructionScript`)