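; BP_Pont is a bridge that rotates once, shortly after play begins, and swaps to a second component.
; BeginPlay hides Pont1, waits, then plays a timeline that drives the world roll of Pivot.
; The timeline's Update also feeds a Delay that hides Pont and shows Pont1, so the visibility swap follows the start of the rotation by a few seconds.
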(event `self.ReceiveBeginPlay`
  (`SceneComponent.SetVisibility` (`self.Pont1`) false false)
  (`KismetSystemLibrary.Delay` 10.0)
  (bind (_direction _newtrack_0) (`Timeline|Timeline_0`)
    (:`Update`
      (`SceneComponent.K2_SetWorldRotation` (`self.Pivot`) (`KismetMathLibrary.MakeRotator` _newtrack_0) false false)
      (`KismetSystemLibrary.Delay` 3.0)
      (`SceneComponent.SetVisibility` (`self.Pont`) false false)
      (`SceneComponent.SetVisibility` (`self.Pont1`) true false))))

(fn `UserConstructionScript`)