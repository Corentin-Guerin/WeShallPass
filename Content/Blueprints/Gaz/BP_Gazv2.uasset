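; Gas zone actor that fades a screen effect on the player's GazPlane when they are exposed to gas without a mask.
; GazZone overlaps set the player's IsInGaz flag and trigger the enter or exit fade.
; Tick also watches mask changes inside the zone, using the player's AnimEnCours flag as a guard.
; After a short delay, each fade creates a dynamic material whose R_Fade and T_Fade parameters are driven by timelines.
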(event `SortieGaz`
  (`KismetSystemLibrary.Delay` 1.5)
  (bind _returnvalue (`PrimitiveComponent.CreateDynamicMaterialInstance` (`/Game/Blueprints/Player/BP_My_Player.GazPlane` (`/Game/Blueprints/Player/FuctionLibrary/BFFL_CallPLayerController.CallMyPlayerCharactere`)) 0 "/Game/Textures/Material/M_GazScreenPlane.M_GazScreenPlane" "None"))
  (`|ExecutionSequence`
    (:`then_0`
      (bind (_direction _newtrack_0) (`Timeline|Timeline_6`)
        (:`Update`
          (`MaterialInstanceDynamic.SetScalarParameterValue` _returnvalue "R_Fade" _newtrack_0))))
    (:`then_1`
      (bind (_direction_2 _newtrack_0_2) (`Timeline|Timeline_7`)
        (:`Update`
          (`MaterialInstanceDynamic.SetScalarParameterValue` _returnvalue "T_Fade" _newtrack_0_2))))))

(event `EntrerGaz`
  (`KismetSystemLibrary.Delay` 1.5)
  (bind _returnvalue (`PrimitiveComponent.CreateDynamicMaterialInstance` (`/Game/Blueprints/Player/BP_My_Player.GazPlane` (`/Game/Blueprints/Player/FuctionLibrary/BFFL_CallPLayerController.CallMyPlayerCharactere`)) 0 "/Game/Textures/Material/M_GazScreenPlane.M_GazScreenPlane" "None"))
  (`|ExecutionSequence`
    (:`then_0`
      (bind (_direction _newtrack_0) (`Timeline|Timeline_4`)
        (:`Update`
          (`MaterialInstanceDynamic.SetScalarParameterValue` _returnvalue "R_Fade" _newtrack_0))))
    (:`then_1`
      (bind (_direction_2 _newtrack_0_2) (`Timeline|Timeline_5`)
        (:`Update`
          (`MaterialInstanceDynamic.SetScalarParameterValue` _returnvalue "T_Fade" _newtrack_0_2))))))

(event `self.ReceiveTick`
  (params (DeltaSeconds :type "Float (single-precision)"))
  (bind _myplayercharactere (`/Game/Blueprints/Player/FuctionLibrary/BFFL_CallPLayerController.CallMyPlayerCharactere`))
  (bind _myplayercharactere_2 (`/Game/Blueprints/Player/FuctionLibrary/BFFL_CallPLayerController.CallMyPlayerCharactere`))
  (bind _returnvalue (not (`/Game/Blueprints/Player/BP_My_Player.AnimEnCours` _myplayercharactere_2)))
  (if (and (not (`/Game/Blueprints/Player/BP_My_Player.IsMasked` _myplayercharactere_2)) (`/Game/Blueprints/Player/BP_My_Player.IsInGaz` _myplayercharactere_2) _returnvalue _returnvalue)
    (set `/Game/Blueprints/Player/BP_My_Player.AnimEnCours` true (`/Game/Blueprints/Player/FuctionLibrary/BFFL_CallPLayerController.CallMyPlayerCharactere`))
    (`self.EntrerGaz`)
    (elif (and (`/Game/Blueprints/Player/BP_My_Player.IsMasked` _myplayercharactere) (`/Game/Blueprints/Player/BP_My_Player.IsInGaz` _myplayercharactere) (`/Game/Blueprints/Player/BP_My_Player.EquipMaskInGaz` _myplayercharactere) (not (`/Game/Blueprints/Player/BP_My_Player.AnimEnCours` _myplayercharactere)))
      (set `/Game/Blueprints/Player/BP_My_Player.AnimEnCours` true (`/Game/Blueprints/Player/FuctionLibrary/BFFL_CallPLayerController.CallMyPlayerCharactere`))
      (`self.SortieGaz`))))

(event `self.GazZone.OnComponentBeginOverlap`
  (params (OverlappedComponent :type "PrimitiveComponent Object Reference") (OtherActor :type "Actor Object Reference") (OtherComp :type "PrimitiveComponent Object Reference") (OtherBodyIndex :type Integer) (bFromSweep :type Boolean) (SweepResult :type "HitResult Structure (by ref)"))
  (bind _myplayercharactere (`/Game/Blueprints/Player/FuctionLibrary/BFFL_CallPLayerController.CallMyPlayerCharactere`))
  (cast `/Game/Blueprints/Player/BP_My_Player` OtherActor)
  (set `/Game/Blueprints/Player/BP_My_Player.IsInGaz` true _myplayercharactere)
  (if (not (`/Game/Blueprints/Player/BP_My_Player.IsMasked` _myplayercharactere))
    (`self.EntrerGaz`)))

(event `self.GazZone.OnComponentEndOverlap`
  (params (OverlappedComponent :type "PrimitiveComponent Object Reference") (OtherActor :type "Actor Object Reference") (OtherComp :type "PrimitiveComponent Object Reference") (OtherBodyIndex :type Integer))
  (bind _myplayercharactere (`/Game/Blueprints/Player/FuctionLibrary/BFFL_CallPLayerController.CallMyPlayerCharactere`))
  (bind _myplayercharactere_2 (`/Game/Blueprints/Player/FuctionLibrary/BFFL_CallPLayerController.CallMyPlayerCharactere`))
  (cast `/Game/Blueprints/Player/BP_My_Player` OtherActor)
  (set `/Game/Blueprints/Player/BP_My_Player.IsInGaz` false _myplayercharactere)
  (if (`/Game/Blueprints/Player/BP_My_Player.IsMasked` _myplayercharactere)
    (set `/Game/Blueprints/Player/BP_My_Player.AnimEnCours` false _myplayercharactere_2)
    (set `/Game/Blueprints/Player/BP_My_Player.EquipMaskInGaz` false _myplayercharactere_2)
    (else
      (set `/Game/Blueprints/Player/BP_My_Player.AnimEnCours` false _myplayercharactere_2)
      (`self.SortieGaz`))))

(fn `UserConstructionScript`)