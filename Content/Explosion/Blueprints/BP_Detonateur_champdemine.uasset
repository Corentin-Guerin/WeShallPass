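; Minefield detonator Blueprint that sets off a group of explosions when a component overlaps its trigger box.
; The overlap event fires three referenced explosions in sequence, each preceded by its own random delay of up to one and a half seconds, staggering the blasts.
; No filter is applied to the overlapping actor, as the player cast is left unconnected.
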(event `self.Triggerbox.OnComponentBeginOverlap`
  (params (OverlappedComponent :type "PrimitiveComponent Object Reference") (OtherActor :type "Actor Object Reference") (OtherComp :type "PrimitiveComponent Object Reference") (OtherBodyIndex :type Integer) (bFromSweep :type Boolean) (SweepResult :type "HitResult Structure (by ref)"))
  (`KismetSystemLibrary.Delay` (`KismetMathLibrary.RandomFloatInRange` 0.0 1.5))
  (`/Game/Explosion/Blueprints/BP_Explosion_2.Explosion` (`self.Explosion`))
  (`KismetSystemLibrary.Delay` (`KismetMathLibrary.RandomFloatInRange` 0.0 1.5))
  (`/Game/Explosion/Blueprints/BP_Explosion_2.Explosion` (`self.Explosion_0`))
  (`KismetSystemLibrary.Delay` (`KismetMathLibrary.RandomFloatInRange` 0.0 1.5))
  (`/Game/Explosion/Blueprints/BP_Explosion_2.Explosion` (`self.Explosion_1`)))

(fn `UserConstructionScript`)