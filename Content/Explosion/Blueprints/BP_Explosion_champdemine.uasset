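; Minefield explosion actor that stages a destructible blast when its Explosion event is called.
; The event adds a destructible component, then after a brief delay fires a radial force impulse, activates particles and plays a sound at world origin.
; It then sets IsExplos and destroys the destructible component after a further delay.
; The IsExplos check against re-triggering is disconnected, so the event runs unguarded.
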(event `Explosion`
  (bind _returnvalue (`AddComponent|NODE_AddDestructibleComponent-0`))
  (`KismetSystemLibrary.Delay` 0.05)
  (`RadialForceComponent.FireImpulse` (`self.RadialForce`))
  (`ActorComponent.Activate` (`self.ParticleSystem`) false)
  (`GameplayStatics.PlaySoundAtLocation` "/Game/StarterContent/Audio/Explosion01.Explosion01" (0.0 0.0 0.0) (struct) 0.5 1.0 0.0 null null null)
  (set `self.IsExplos` true)
  (`KismetSystemLibrary.Delay` 2.0)
  (`ActorComponent.K2_DestroyComponent` _returnvalue))

(fn `UserConstructionScript`)